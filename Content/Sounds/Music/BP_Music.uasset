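; BP_Music is a music manager that plays a 2D track from BeginPlay and responds to a bound ChangeMusic event.
; The first change spawns a second persistent sound component with the new track and toggles the starting one off.
; Later changes only toggle both components' active state to alternate between them, storing the passed track in MusicToPlay without spawning or assigning it.
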(event Custom|Change%20Music
  (params (New%20Music :type Sound%20Base%20Object%20Reference))
  (bind _output_get (Variables|Default|SetMusicToPlay New%20Music))
  (if (not (Variables|Default|GetisFirstSongActive?))
    (bind _returnvalue (Audio|SpawnSound2D _output_get 1.0 1.0 0.0 0 false false))
    (Variables|Default|SetSecondSound _returnvalue)
    (Components|Activation|ToggleActive (Variables|Default|GetStartSound))
    (Variables|Default|SetisFirstSongActive? true)
    (else
      (Components|Activation|ToggleActive (Variables|Default|GetSecondSound))
      (Components|Activation|ToggleActive (Variables|Default|GetStartSound)))))

(event EventBeginPlay
  (bind _returnvalue (Audio|SpawnSound2D (Variables|Default|GetMusicToPlay) 1.0 1.0 0.0 0 false false))
  (Variables|Default|SetStartSound _returnvalue)
  (EventDispatchers|BindEventtoChangeMusic (delegate Custom|Change%20Music)))

(fn ConstructionScript)