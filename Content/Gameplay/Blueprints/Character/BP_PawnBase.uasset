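; Base player pawn for a lane-based runner with lane switching, jumping, attacking and a 15-second coin magnet state.
; Init takes lane count and width from the level manager, which also gates input on IsPlaying.
; Timelines lerp lane moves and jumps, guarded by DoOnce nodes and state flags, with the spring arm held at fixed height during jumps.
; Helper functions play the lose animation and blend the intro camera.
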(event Custom|CoinMagnetCollected
  (Variables|Default|SetCoinMagnetOn? true)
  (Utilities|FlowControl|Delay 15.0)
  (Variables|Default|SetCoinMagnetOn? false))

(event EventBeginPlay
  (CallFunction|Init))

(event Input|ActionEvents|InputActionLeft
  (params (Key :type Key%20Structure :default "None"))
  (bind _returnvalue (Transformation|GetActorLocation))
  (bind _skeletalmesh (Variables|Default|GetSkeletalMesh))
  (bind _skeletalmesh_2 (Variables|Default|GetSkeletalMesh))
  (bind _relativerotation (Variables|/Script/Engine.SceneComponent|GetRelativeRotation _skeletalmesh))
  (bind _relativerotation_2 (Variables|/Script/Engine.SceneComponent|GetRelativeRotation _skeletalmesh_2))
  (:Pressed
    (if (Variables|/Game/Gameplay/Blueprints/Game/BP_LevelManager.BP_LevelManager_C|GetbIsPlaying (Variables|Default|GetLevelManagerRef))
      ;[1 1 1] Pressed Left whilst in Left most lane
      (if (not (<= (Variables|Default|GetCurrentLane) 1))
        (if (not (Variables|Default|GetIsMovingRight?))
          (Variables|Default|SetIsMovingLeft? true)
          (if (Variables|Default|GetbMoving)
            (if (Variables|Default|GetIsJumping?)
              (Variables|Default|SetbMoving true :!label _label)
              (Utilities|FlowControl|DoOnce false :!label _label_2
                (:Completed
                  (Variables|Default|SetTargetPosition (- (.y (Transformation|GetActorLocation)) (Variables|Default|GetLaneWidth)))
                  (Transformation|SetRelativeRotation _skeletalmesh (Math|Rotator|MakeRotator (.roll _relativerotation) (.pitch _relativerotation) (Math|Float|Lerp (.yaw _relativerotation) (- (.yaw _relativerotation) 3e+01) 1.0)) false false)
                  (bind _move (Timeline|MoveLeft PlayFromStart)
                    (:Update
                      (Transformation|SetActorLocation (Math|Vector|MakeVector (.x _returnvalue) (Math|Float|Lerp (.y _returnvalue) (Variables|Default|GetTargetPosition) _move) (.z _returnvalue)) false false))
                    (:Finished
                      (Variables|Default|SetIsMovingLeft? false)
                      (Variables|Default|SetbMoving false)
                      (Math|Integer|DecrementInt (Variables|Default|GetCurrentLane)
                        (:%20%20
                          (Transformation|SetRelativeRotation _skeletalmesh_2 (Math|Rotator|MakeRotator (.roll _relativerotation_2) (.pitch _relativerotation_2) (Math|Float|Lerp (.yaw _relativerotation_2) (+ (.yaw _relativerotation_2) 3e+01) 1.0)) false false)
                          (goto _label_2 Reset))))))))
            (else
              (goto _label))))))))

(event Input|ActionEvents|InputActionRight
  (params (Key :type Key%20Structure :default "None"))
  (bind _returnvalue (Transformation|GetActorLocation))
  (bind _skeletalmesh (Variables|Default|GetSkeletalMesh))
  (bind _skeletalmesh_2 (Variables|Default|GetSkeletalMesh))
  (bind _relativerotation (Variables|/Script/Engine.SceneComponent|GetRelativeRotation _skeletalmesh))
  (bind _relativerotation_2 (Variables|/Script/Engine.SceneComponent|GetRelativeRotation _skeletalmesh_2))
  (:Pressed
    (if (Variables|/Game/Gameplay/Blueprints/Game/BP_LevelManager.BP_LevelManager_C|GetbIsPlaying (Variables|Default|GetLevelManagerRef))
      ;[1 1 1] Pressed Right whilst in the Right most lane
      (if (not (== (Variables|Default|GetCurrentLane) (Variables|/Game/Gameplay/Blueprints/Game/BP_LevelManager.BP_LevelManager_C|GetNumberOfLanes (Variables|Default|GetLevelManagerRef))))
        (if (not (Variables|Default|GetIsMovingLeft?))
          (Variables|Default|SetIsMovingRight? true)
          (if (Variables|Default|GetbMoving)
            (if (Variables|Default|GetIsJumping?)
              (Variables|Default|SetbMoving true :!label _label)
              (Utilities|FlowControl|DoOnce false :!label _label_2
                (:Completed
                  (Variables|Default|SetTargetPosition (+ (.y (Transformation|GetActorLocation)) (Variables|Default|GetLaneWidth)))
                  (Transformation|SetRelativeRotation _skeletalmesh (Math|Rotator|MakeRotator (.roll _relativerotation) (.pitch _relativerotation) (Math|Float|Lerp (.yaw _relativerotation) (+ (.yaw _relativerotation) 3e+01) 1.0)) false false)
                  (bind _move (Timeline|MoveRight PlayFromStart)
                    (:Update
                      (Transformation|SetActorLocation (Math|Vector|MakeVector (.x _returnvalue) (Math|Float|Lerp (.y _returnvalue) (Variables|Default|GetTargetPosition) _move) (.z _returnvalue)) false false))
                    (:Finished
                      (Variables|Default|SetIsMovingRight? false)
                      (Variables|Default|SetbMoving false)
                      (Math|Integer|IncrementInt (Variables|Default|GetCurrentLane)
                        (:%20%20
                          (Transformation|SetRelativeRotation _skeletalmesh_2 (Math|Rotator|MakeRotator (.roll _relativerotation_2) (.pitch _relativerotation_2) (Math|Float|Lerp (.yaw _relativerotation_2) (- (.yaw _relativerotation_2) 3e+01) 1.0)) false false)
                          (goto _label_2 Reset))))))))
            (else
              (goto _label))))))))

(event Input|ActionEvents|InputActionJump
  (params (Key :type Key%20Structure :default "None"))
  (bind _returnvalue (Transformation|GetActorLocation))
  (bind _returnvalue_2 (Transformation|GetActorLocation))
  (bind _springarm (Variables|Default|GetSpringArm))
  (bind _springarm_2 (Variables|Default|GetSpringArm))
  (bind _returnvalue_3 (Transformation|GetWorldLocation _springarm))
  (bind _returnvalue_4 (Transformation|GetWorldLocation _springarm_2))
  (:Pressed
    (if (Variables|/Game/Gameplay/Blueprints/Game/BP_LevelManager.BP_LevelManager_C|GetbIsPlaying (Variables|Default|GetLevelManagerRef))
      (if (not (or (and (Variables|Default|GetIsJumping?) (Variables|Default|GetbMoving)) (Variables|Default|GetIsAttacking?)))
        (Utilities|FlowControl|DoOnce false :!label _label
          (:Completed
            (Variables|Default|SetIsJumping? true)
            (Variables|Default|SetbMoving true)
            (bind _move (Timeline|Jump%20Up PlayFromStart)
              (:Update
                (Transformation|SetActorLocation (Math|Vector|MakeVector 0.0 (.y _returnvalue) (Math|Float|Lerp (.z _returnvalue) 3.5e+02 _move)) false false)
                (Transformation|SetWorldLocation _springarm_2 (Math|Vector|MakeVector (.x _returnvalue_4) (.y _returnvalue_4) 1e+02) false false))
              (:Finished
                (Utilities|FlowControl|Delay 0.4)
                (Variables|Default|SetIsJumping? false)
                (Variables|Default|SetbMoving false)
                (bind _move_2 (Timeline|Jump%20Down PlayFromStart)
                  (:Update
                    (Transformation|SetActorLocation (Math|Vector|MakeVector (.x _returnvalue_2) (.y _returnvalue_2) (Math|Float|Lerp (.z _returnvalue_2) 1e+02 _move_2)) false false)
                    (Transformation|SetWorldLocation _springarm (Math|Vector|MakeVector (.x _returnvalue_3) (.y _returnvalue_3) 1e+02) false false))
                  (:Finished
                    (goto _label Reset)))))))))))

(event Input|ActionEvents|InputActionAttack
  (params (Key :type Key%20Structure :default "None"))
  (:Pressed
    (if (Variables|/Game/Gameplay/Blueprints/Game/BP_LevelManager.BP_LevelManager_C|GetbIsPlaying (Variables|Default|GetLevelManagerRef))
      (Utilities|FlowControl|DoOnce false :!label _label
        (:Completed
          (Variables|Default|SetIsAttacking? true)
          (Animation|Montage|PlayMontage (Variables|Default|GetSkeletalMesh) "/Game/Gameplay/Blueprints/Character/Anim_Attack_Montage_Char.Anim_Attack_Montage_Char"
            (:OnCompleted
              (Variables|Default|SetIsAttacking? false)
              (goto _label Reset))))))))

(fn ConstructionScript)

(fn Init
  (bind (_levelmanager _levelmanagerfound) (CallFunction|GetLevelManager))
  (if _levelmanagerfound
    (Variables|Default|SetLevelManagerRef _levelmanager)
    (Variables|Default|SetCurrentLane (+ (/ (Variables|/Game/Gameplay/Blueprints/Game/BP_LevelManager.BP_LevelManager_C|GetNumberOfLanes (Variables|Default|GetLevelManagerRef)) 2) 1))
    (Variables|Default|SetLaneWidth (Variables|/Game/Gameplay/Blueprints/Game/BP_LevelManager.BP_LevelManager_C|GetLaneWidth (Variables|Default|GetLevelManagerRef)))
    (else
      (Development|PrintString "No Level Manager Found"))))

(fn HitObstacle
  (Variables|Default|SetIsRunning? false)
  (Components|Animation|PlayAnimation (Variables|Default|GetSkeletalMesh) "/Game/UndeadPack/EnemyGoblin/Animations/Anim_Lose.Anim_Lose" false))

(fn CameraStartSetUp
  (params (Time :type Float%20%28single-precision%29))
  (bind _springarm (Variables|Default|GetSpringArm))
  (Variables|/Script/Engine.SpringArmComponent|SetTargetArmLength (Variables|Default|GetSpringArm) (Math|Float|Lerp 3e+02 8e+02 Time))
  (Transformation|SetWorldRotation _springarm (Math|Rotator|MakeRotator (.roll (Transformation|GetWorldRotation _springarm)) (Math|Float|Lerp -15.0 -4e+01 Time) (Math|Float|Lerp 195.0 0.0 Time)) false false))