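; Game mode for a goblin runner, driving start screen, pre-game intro, play and post-game phases.
; It takes spawners and Lich from the level manager, plays intro effects and a camera-turn timeline, then starts level movement.
; Looping timers track time and drive timeline-lerped score, with a multiplier that doubles at escalating goals.
; Post-game runs once, showing the end popup and saving score, coins, kills and high score to the game instance.
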(event Custom|Set-Up
  (bind _level_manager (Variables|Default|GetLevel%20Manager))
  (Variables|/Game/Gameplay/Blueprints/Game/BP_LevelManager.BP_LevelManager_C|SetLevelSpeed _level_manager 0.0)
  (Variables|/Game/Gameplay/Blueprints/Game/BP_LevelManager.BP_LevelManager_C|SetbIsPlaying _level_manager false)
  (bind _returnvalue (UserInterface|CreateWidget "/Game/UI/StartScreen.StartScreen_C"))
  (bind _output_get (Variables|Default|SetStartScreen _returnvalue))
  (UserInterface|Viewport|AddtoViewport _output_get 0))

(event Custom|CameraTurn
  (bind _returnvalue (Game|GetPlayerController 0))
  (bind _as_bp_pawn_base (Variables|Default|GetAs%20BP%20Pawn%20Base))
  ;[1 1 1] Camera Spin
  (bind _time (Timeline|StartCameraMove PlayFromStart)
    (:Update
      (Default|CameraStartSetUp _as_bp_pawn_base _time)
      (Input|DisableInput _as_bp_pawn_base _returnvalue))
    (:Finished
      (Input|EnableInput _as_bp_pawn_base _returnvalue))))

(event Custom|In-Game
  (bind _level_manager (Variables|Default|GetLevel%20Manager))
  (Variables|/Game/Gameplay/Blueprints/Game/BP_LevelManager.BP_LevelManager_C|SetLevelSpeed _level_manager -5e+02)
  (Variables|/Game/Gameplay/Blueprints/Game/BP_LevelManager.BP_LevelManager_C|SetbIsPlaying _level_manager true)
  (Variables|/Game/Gameplay/Blueprints/Character/BP_PawnBase.BP_PawnBase_C|SetIsRunning? (Variables|Default|GetAs%20BP%20Pawn%20Base) true)
  (Default|LineUpNextObstacleSpawn (Variables|Default|GetLeft%20Side%20Obstacle%20Spawner%20Ref))
  (Default|LineUpNextObstacleSpawn (Variables|Default|GetRight%20Side%20Obstacle%20Spawner%20Ref))
  (Default|DestroyScenery (Variables|/Game/Gameplay/Blueprints/Game/BP_LevelManager.BP_LevelManager_C|GetBackground (Variables|Default|GetLevel%20Manager)))
  (bind _returnvalue (Utilities|Time|SetTimerbyEvent (delegate Custom|StartScoring) 0.1 true))
  (Variables|Default|SetScoreTimer _returnvalue)
  (bind _returnvalue_2 (Utilities|Time|SetTimerbyEvent (delegate Custom|GameTimer) 1.0 true))
  (Variables|Default|SetTimer _returnvalue_2))

(event Custom|StartScoring
  (Variables|Default|SetCurrentScore (Variables|Default|GetTotalScore))
  (bind _lerp (Timeline|LerpScore PlayFromStart)
    (:Update
      (CallFunction|CalculateScore (Variables|Default|GetSpeed) _lerp))))

(event Custom|Post-Game
  (bind _returnvalue (Game|GetGameInstance))
  (bind _returnvalue_2 (Game|GetGameInstance))
  (bind _asbp_game_instance (Utilities|Casting|CastToBP_GameInstance _returnvalue))
  (bind _asbp_game_instance_2 (Utilities|Casting|CastToBP_GameInstance _returnvalue_2))
  (Utilities|FlowControl|DoOnce false
    (:Completed
      (Default|CallChangeMusic (Variables|/Game/Gameplay/Blueprints/Game/BP_LevelManager.BP_LevelManager_C|GetMusicControl (Variables|Default|GetLevel%20Manager)) "/Game/Sounds/Music/creepy-pecan-pie-main-version-00-37-8836_Cue.creepy-pecan-pie-main-version-00-37-8836_Cue")
      (Utilities|Time|ClearandInvalidateTimerbyHandle (Variables|Default|GetScoreTimer))
      (Utilities|Time|ClearandInvalidateTimerbyHandle (Variables|Default|GetTimer))
      (CallFunction|CalculateDistanceTravelled)
      (bind _returnvalue_3 (UserInterface|CreateWidget "/Game/UI/EndPopUp.EndPopUp_C"))
      (UserInterface|Viewport|AddtoViewport _returnvalue_3 0)
      (Variables|/Game/Gameplay/Blueprints/Game/BP_GameInstance.BP_GameInstance_C|SetRecentScore _asbp_game_instance_2 (Variables|Default|GetTotalScore))
      (Variables|/Game/Gameplay/Blueprints/Game/BP_GameInstance.BP_GameInstance_C|SetTotalCoins _asbp_game_instance_2 (+ (Variables|/Game/Gameplay/Blueprints/Game/BP_GameInstance.BP_GameInstance_C|GetTotalCoins _asbp_game_instance_2) (Variables|Default|GetCoins)))
      (Variables|/Game/Gameplay/Blueprints/Game/BP_GameInstance.BP_GameInstance_C|SetTotalKills _asbp_game_instance (+ (Variables|/Game/Gameplay/Blueprints/Game/BP_GameInstance.BP_GameInstance_C|GetTotalKills _asbp_game_instance_2) (Variables|Default|GetKills)))
      (if (> (Variables|Default|GetTotalScore) (Variables|/Game/Gameplay/Blueprints/Game/BP_GameInstance.BP_GameInstance_C|GetHighScore _asbp_game_instance))
        (Variables|/Game/Gameplay/Blueprints/Game/BP_GameInstance.BP_GameInstance_C|SetHighScore _asbp_game_instance (Variables|Default|GetTotalScore))))))

(event Custom|GameTimer
  (bind _output_get (Variables|Default|SetSeconds (+ (Variables|Default|GetSeconds) 1.0)))
  (if (> _output_get 59.0)
    (bind _result (Math|Integer|IncrementInt (Variables|Default|GetMinutes))
      (:%20%20
        (Variables|Default|SetMinutes _result)
        (Variables|Default|SetSeconds 0.0)))))

(event Custom|Pre-Game
  (Default|SpawnLich (Variables|Default|GetLich%20Ref))
  (Default|CallChangeMusic (Variables|/Game/Gameplay/Blueprints/Game/BP_LevelManager.BP_LevelManager_C|GetMusicControl (Variables|Default|GetLevel%20Manager)) "/Game/Sounds/Music/happy-comedy-halloween-party-dance-for-kids-children-118581_WAV_Cue.happy-comedy-halloween-party-dance-for-kids-children-118581_WAV_Cue")
  (Utilities|FlowControl|Delay 1.77)
  (Default|GoblinScream (Variables|Default|GetAs%20BP%20Pawn%20Base))
  (Utilities|FlowControl|Delay 1.5)
  (bind _returnvalue (UserInterface|CreateWidget "/Game/UI/HUD.HUD_C"))
  (bind _output_get (Variables|Default|SetHUD _returnvalue))
  (UserInterface|Viewport|AddtoViewport _output_get 0)
  (CallFunction|CameraTurn)
  (Default|LineUpNextObstacleSpawn (Variables|/Game/Gameplay/Blueprints/Game/BP_LevelManager.BP_LevelManager_C|GetNewSpawner (Variables|Default|GetLevel%20Manager)))
  (CallFunction|In-Game))

(event Custom|Init
  (bind (_levelmanager _levelmanagerfound) (CallFunction|GetLevelManager))
  (if _levelmanagerfound
    (Variables|Default|SetLevel%20Manager _levelmanager)
    (bind _asbp_pawn_base (Utilities|Casting|CastToBP_PawnBase (Game|Player|GetPlayerPawn 0)))
    (Variables|Default|SetAs%20BP%20Pawn%20Base _asbp_pawn_base)
    (Variables|Default|SetLich%20Ref (Variables|/Game/Gameplay/Blueprints/Game/BP_LevelManager.BP_LevelManager_C|GetLichRef (Variables|Default|GetLevel%20Manager)))
    (Variables|Default|SetObstacle%20Spawner%20Ref (Variables|/Game/Gameplay/Blueprints/Game/BP_LevelManager.BP_LevelManager_C|GetObstacleSpawnerRef (Variables|Default|GetLevel%20Manager)))
    (Variables|Default|SetLeft%20Side%20Obstacle%20Spawner%20Ref (Variables|/Game/Gameplay/Blueprints/Game/BP_LevelManager.BP_LevelManager_C|GetLeftSideObstacleSpawnerRef (Variables|Default|GetLevel%20Manager)))
    (Variables|Default|SetRight%20Side%20Obstacle%20Spawner%20Ref (Variables|/Game/Gameplay/Blueprints/Game/BP_LevelManager.BP_LevelManager_C|GetRightSideObstacleSpawnerRef (Variables|Default|GetLevel%20Manager)))))

(event EventBeginPlay
  (CallFunction|Init)
  (CallFunction|Set-Up))

(fn ConstructionScript)

(fn AddKillPoints
  (Variables|Default|SetKills (+ (Variables|Default|GetKills) 1)))

(fn AddCoins
  (Variables|Default|SetCoins (+ (Variables|Default|GetCoins) 1)))

(fn AddtoScore
  (params (PointsToAdd :type Float%20%28single-precision%29))
  (Variables|Default|SetTotalScore (+ PointsToAdd (Variables|Default|GetTotalScore))))

(fn CalculateScore
  (params (Speed :type Float%20%28single-precision%29) (Lerp :type Float%20%28single-precision%29))
  (Variables|Default|SetTotalScore (Math|Float|Lerp (Variables|Default|GetCurrentScore) (+ (Variables|Default|GetTotalScore) (* Speed (Variables|Default|GetScoreMulitplyer))) Lerp))
  (if (>= (Variables|Default|GetTotalScore) (Variables|Default|GetMultiplyerScoreGoal))
    (Variables|Default|SetScoreMulitplyer (* (Variables|Default|GetScoreMulitplyer) 2.0))
    (Variables|Default|SetPreviousGoal (Variables|Default|GetMultiplyerScoreGoal))
    (Variables|Default|SetMultiplyerScoreGoal (* (Variables|Default|GetMultiplyerScoreGoal) (Variables|Default|GetGoalIncreaseMultiplyer)))
    (Variables|Default|SetGoalIncreaseMultiplyer (* (Variables|Default|GetGoalIncreaseMultiplyer) 2.0))
    (Default|CallScoreUpdated)
    (else
      (Default|CallScoreUpdated))))

(fn CalculateDistanceTravelled
  (Variables|Default|SetDistance (* (* (Variables|Default|GetSpeed) 1e+01) (Variables|Default|GetSeconds))))