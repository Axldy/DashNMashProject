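; Player controller for the endless runner that opens and closes the Settings menu with Escape, except once the run has ended.
; Escape checks the end-of-run flag on BP_GameModeBase, then calls SettingsToggle, where a FlipFlop alternates between opening and closing.
; The first open creates the widget and adds it to the viewport; later toggles reuse it, switching visibility and tracking IsSettingsOpened.
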(event Custom|SettingsToggle
  (Utilities|FlowControl|FlipFlop
    (:A
      (Utilities|FlowControl|Sequence
        (:then_0
          (Utilities|FlowControl|DoOnce false
            (:Completed
              (bind _returnvalue (UserInterface|CreateWidget "/Game/UI/Settings.Settings_C"))
              (bind _output_get (Variables|Default|SetSettings _returnvalue))
              (UserInterface|Viewport|AddtoViewport _output_get 0))))
        (:then_1
          (Default|OpenWidget (Variables|Default|GetSettings))
          (Variables|Default|SetisSettingsOpened? true)
          (Widget|SetVisibility (Variables|Default|GetSettings) "Visible"))))
    (:B
      (Default|RemovefromHUD (Variables|Default|GetSettings))
      (Widget|SetVisibility (Variables|Default|GetSettings) "Hidden")
      (Variables|Default|SetisSettingsOpened? false))))

(event Input|KeyboardEvents|Escape
  (params (Key :type Key%20Structure :default "None"))
  (:Pressed
    (if (not (Variables|/Game/Gameplay/Blueprints/Game/BP_GameModeBase.BP_GameModeBase_C|GetisEndOfRun? (.AsBP%20Game%20Mode%20Base (Utilities|Casting|CastToBP_GameModeBase (Game|GetGameMode)))))
      (Utilities|FlowControl|DoOnce false :!label _label
        (:Completed
          (CallFunction|SettingsToggle)
          (goto _label Reset))))))

(fn ConstructionScript)