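; Floor side-asset actor, named for the left side, that scatters a few instanced static meshes at random points within its Box.
; The Construction Script moves the instanced mesh component to the Box's relative location as a world position, clears it, then adds instances using random points from the Box bounds.
; Instances keep unit scale, the random-range nodes are unused, and the event graph has no active logic.
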(event EventBeginPlay)

(event Collision|EventActorBeginOverlap
  (params (OtherActor :type Actor%20Object%20Reference)))

(event EventTick
  (params (DeltaSeconds :type Float%20%28single-precision%29)))

(fn ConstructionScript
  (bind _box (Variables|Default|GetBox))
  (bind (_origin _boxextent) (Collision|GetComponentBounds _box))
  (bind _returnvalue (Math|Random|RandomPointinBoundingBox _origin _boxextent))
  (|CallParentFunction)
  (Transformation|SetWorldLocation (Variables|Default|GetInstancedStaticMesh) (Variables|/Script/Engine.SceneComponent|GetRelativeLocation (Variables|Default|GetBox)) false false)
  (Components|InstancedStaticMesh|ClearInstances (Variables|Default|GetInstancedStaticMesh))
  (for _index (range 0 2)
    (Components|InstancedStaticMesh|AddInstance (Variables|Default|GetInstancedStaticMesh) (Math|Transform|MakeTransform (Math|Vector|MakeVector (.x _returnvalue) (.y _returnvalue) (.z _returnvalue)) "0, 0, 0" (Math|Vector|MakeVector 1.0 1.0 1.0)))))