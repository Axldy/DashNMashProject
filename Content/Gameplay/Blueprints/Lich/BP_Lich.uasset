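; BP_Lich is the Lich character Blueprint, handling its staged entrance through a portal.
; SpawnLich shows the portal, scales it with a timeline, then plays the emergence montage with a laugh sound and briefly delayed mesh reveal.
; When the montage completes, a second timeline rescales the portal, which is then hidden as IsRunning becomes true.
; BeginPlay caches a Level Manager reference, printing a message if none is found.
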(event Custom|SpawnLich
  (bind _portal (Variables|Default|GetPortal))
  (bind _portal_2 (Variables|Default|GetPortal))
  (bind _returnvalue (Transformation|GetRelativeTransform _portal_2))
  (bind _returnvalue_2 (Transformation|GetRelativeTransform _portal))
  (Rendering|SetVisibility (Variables|Default|GetPortal) true false)
  (bind _scale (Timeline|ScalePortal Play)
    (:Update
      (Transformation|SetRelativeTransform _portal (Math|Transform|MakeTransform (.location _returnvalue_2) (.rotation _returnvalue_2) _scale) false false))
    (:Finished
      (Animation|Montage|PlayMontage (Variables|Default|GetSkeletalMesh) "/Game/Gameplay/Blueprints/Lich/Anim_Emergence_Montage.Anim_Emergence_Montage"
        (:then
          (Audio|PlaySoundatLocation "/Game/Sounds/SFX/LichLaugh.LichLaugh" (Transformation|GetWorldLocation (Variables|Default|GetSkeletalMesh)) "0, 0, 0" 1.0 1.0 0.0 0 0 0)
          (Utilities|FlowControl|Delay 0.3)
          (Rendering|SetVisibility (Variables|Default|GetSkeletalMesh) true false))
        (:OnCompleted
          (bind _newtrack_0 (Timeline|Timeline_0 Play)
            (:Update
              (Transformation|SetRelativeTransform _portal_2 (Math|Transform|MakeTransform (.location _returnvalue) (.rotation _returnvalue) _newtrack_0) false false))
            (:Finished
              (Variables|Default|SetIsRunning? true)
              (Rendering|SetVisibility (Variables|Default|GetPortal) false false))))))))

(event EventBeginPlay
  (CallFunction|Init))

(fn ConstructionScript)

(fn Init
  (bind (_levelmanager _levelmanagerfound) (CallFunction|GetLevelManager))
  (if _levelmanagerfound
    (Variables|Default|SetLevelManagerRef _levelmanager)
    (else
      (Development|PrintString "No Level Manager Found"))))