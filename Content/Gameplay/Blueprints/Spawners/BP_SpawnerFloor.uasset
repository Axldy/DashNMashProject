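; BP_SpawnerFloor is a child spawner that builds a row of floor tiles along X and recycles them to keep the floor continuous.
; On BeginPlay it spawns the required number through the parent's SpawnActor, starting at its own location and spacing them by a hardcoded tile size while tracking the rear tile.
; When a tile hits bounds, it waits briefly, moves that tile behind RearTile and makes it the new rear.
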(event EventBeginPlay
  (|CallParentFunction)
  (for _index (range 0 (Variables|Default|GetActorsRequiredCount))
    (if (== _index 0)
      (bind _returnvalue (CallFunction|SpawnActor))
      (Variables|Default|SetRearTile _returnvalue)
      (Variables|Default|SetTileSize 8e+02)
      (Transformation|SetActorLocation (Variables|Default|GetRearTile) (Transformation|GetActorLocation) false false)
      (else
        (bind _returnvalue_2 (CallFunction|SpawnActor))
        (Transformation|SetActorLocation _returnvalue_2 (Math|Vector|MakeVector (+ (.x (Transformation|GetActorLocation (Variables|Default|GetRearTile))) (Variables|Default|GetTileSize)) (.y (Transformation|GetActorLocation (Variables|Default|GetRearTile))) 0.0) false false)
        (Variables|Default|SetRearTile _returnvalue_2)))))

(event EventSpawnedActorHitBounds
  (params (OutOfBoundsActor :type Actor%20Object%20Reference))
  (Utilities|FlowControl|Delay 0.01)
  (Transformation|SetActorLocation OutOfBoundsActor (Math|Vector|MakeVector (+ (.x (Transformation|GetActorLocation (Variables|Default|GetRearTile))) (Variables|Default|GetTileSize)) (.y (Transformation|GetActorLocation (Variables|Default|GetRearTile))) (.z (Transformation|GetActorLocation (Variables|Default|GetRearTile)))) false false)
  (Variables|Default|SetRearTile OutOfBoundsActor))

(fn ConstructionScript
  (|CallParentFunction))

(fn SpawnActor
  (bind _returnvalue (|CallParentFunction))
  (return _returnvalue))