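; Obstacle spawner that streams farm, village and forest obstacles during play, grouped into themed areas with entry and exit pieces.
; BeginPlay picks a random entry piece, then a self-calling, random-delay loop places obstacles at the spawner while LevelManager is playing.
; Each spawn decrements a counter to choose the next class: random area piece, exit, or a different area's entry, re-rolling repeats.
; Actors reported out of bounds are destroyed.
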(event Custom|LineUpNextObstacleSpawn
  (Utilities|FlowControl|Delay (Math|Random|RandomFloatinRange (Variables|Default|GetMinDelay) (Variables|Default|GetMaxDelay)))
  (CallFunction|PlaceObstacle)
  (if (Variables|/Game/Gameplay/Blueprints/Game/BP_LevelManager.BP_LevelManager_C|GetbIsPlaying (Variables|Default|GetLevelManagerRef))
    (CallFunction|LineUpNextObstacleSpawn)))

(event EventSpawnedActorHitBounds
  (params (OutOfBoundsActor :type Actor%20Object%20Reference))
  (Actor|DestroyActor OutOfBoundsActor))

(event EventBeginPlay
  (bind (_levelmanager _levelmanagerfound) (CallFunction|GetLevelManager))
  (if _levelmanagerfound
    (Variables|Default|SetLevelManagerRef _levelmanager)
    (switch int (Math|Random|RandomIntegerinRange 0 2)
      (:0
        (Variables|Default|SetObstacle "/Game/Gameplay/Blueprints/Obstacles/Obstacle_Test/Farm/Obstacle_Farm_Entry.Obstacle_Farm_Entry_C"))
      (:1
        (Variables|Default|SetObstacle "/Game/Gameplay/Blueprints/Obstacles/Obstacle_Test/Forest/ObstacleForestEntry.ObstacleForestEntry_C"))
      (:2
        (Variables|Default|SetObstacle "/Game/Gameplay/Blueprints/Obstacles/Obstacle_Test/Villiage/ObstacleVillageEntry.ObstacleVillageEntry_C")))
    (CallFunction|LineUpNextObstacleSpawn)))

(fn ConstructionScript
  (|CallParentFunction))

(fn PlaceObstacle
  (bind _returnvalue (CallFunction|SpawnActor))
  (Utilities|IsValid _returnvalue
    (:Is%20Valid
      (Transformation|SetActorLocation _returnvalue (Transformation|GetActorLocation) false false))))

(fn SpawnActor
  (bind _returnvalue (Game|SpawnActorfromClass (Variables|Default|GetObstacle) (Math|Transform|MakeTransform "0.000000,0.000000,-1000.000000" "0, 0, 0" "1,1,1") "Undefined" 0 0))
  (Default|GetSpawnerRef _returnvalue self)
  (Variables|Default|SetCurrentAreaType (Variables|/Game/Gameplay/Blueprints/Obstacles/Obstacle_Test/ObstacleBase.ObstacleBase_C|GetAreaType _returnvalue))
  (CallFunction|ObstacleSpawning)
  (Class|BPISpawnable|SetParent(Message) _returnvalue self)
  (return _returnvalue))

(fn ObstacleSpawning
  (bind _result (Math|Integer|DecrementInt (Variables|Default|GetAreaSpawnCount))
    (:%20%20
      (bind _output_get (Variables|Default|SetAreaSpawnCount _result))
      (if (== _output_get 0)
        ;[1 1 1] Change Area
        (switch int (Math|Random|RandomIntegerinRange 0 2) :!label _label
          (:0
            (bind _output_get_2 (Variables|Default|SetNextAreaType "NewEnumerator0"))
            (if (Utilities|Enum|Equal(Enum) _output_get_2 (Variables|Default|GetCurrentAreaType))
              (goto _label)
              (else
                (Variables|Default|SetObstacle "/Game/Gameplay/Blueprints/Obstacles/Obstacle_Test/Farm/Obstacle_Farm_Entry.Obstacle_Farm_Entry_C")
                (Variables|Default|SetAreaSpawnCount 10))))
          (:1
            (bind _output_get_3 (Variables|Default|SetNextAreaType "NewEnumerator1"))
            (if (Utilities|Enum|Equal(Enum) _output_get_3 (Variables|Default|GetCurrentAreaType))
              (goto _label)
              (else
                (Variables|Default|SetObstacle "/Game/Gameplay/Blueprints/Obstacles/Obstacle_Test/Villiage/ObstacleVillageEntry.ObstacleVillageEntry_C")
                (Variables|Default|SetAreaSpawnCount 10))))
          (:2
            (bind _output_get_4 (Variables|Default|SetNextAreaType "NewEnumerator2"))
            (if (Utilities|Enum|Equal(Enum) _output_get_4 (Variables|Default|GetCurrentAreaType))
              (goto _label)
              (else
                (Variables|Default|SetObstacle "/Game/Gameplay/Blueprints/Obstacles/Obstacle_Test/Forest/ObstacleForestEntry.ObstacleForestEntry_C")
                (Variables|Default|SetAreaSpawnCount 10)))))
        (else
          ;[1 1 1] Check Final Tile
          (if (== (Variables|Default|GetAreaSpawnCount) 1)
            (if (Utilities|Enum|Equal(Enum) (Variables|Default|GetCurrentAreaType) "NewEnumerator0")
              (Variables|Default|SetObstacle "/Game/Gameplay/Blueprints/Obstacles/Obstacle_Test/Farm/Obstacle_Farm_Exit.Obstacle_Farm_Exit_C")
              (elif (Utilities|Enum|Equal(Enum) (Variables|Default|GetCurrentAreaType) "NewEnumerator1")
                (Variables|Default|SetObstacle "/Game/Gameplay/Blueprints/Obstacles/Obstacle_Test/Villiage/ObstacleVillageExit1.ObstacleVillageExit1_C")
                (elif (Utilities|Enum|Equal(Enum) (Variables|Default|GetCurrentAreaType) "NewEnumerator2")
                  (Variables|Default|SetObstacle "/Game/Gameplay/Blueprints/Obstacles/Obstacle_Test/Forest/ObstacleForestExit1.ObstacleForestExit1_C"))))
            (else
              ;[1 1 1] Set New Obstacles
              (if (Utilities|Enum|Equal(Enum) (Variables|Default|GetCurrentAreaType) "NewEnumerator0")
                (Variables|Default|SetObstacle (Utilities|Array|Get(acopy) (Variables|Default|GetFarmArea) (Math|Random|RandomIntegerinRange 2 3)))
                (elif (Utilities|Enum|Equal(Enum) (Variables|Default|GetCurrentAreaType) "NewEnumerator1")
                  (Variables|Default|SetObstacle (Utilities|Array|Get(acopy) (Variables|Default|GetVillageArea) (Math|Random|RandomIntegerinRange 2 3)))
                  (elif (Utilities|Enum|Equal(Enum) (Variables|Default|GetCurrentAreaType) "NewEnumerator2")
                    (Variables|Default|SetObstacle (Utilities|Array|Get(acopy) (Variables|Default|GetForestArea) (Math|Random|RandomIntegerinRange 2 3)))))))))))))