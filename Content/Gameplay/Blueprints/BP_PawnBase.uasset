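; BP_PawnBase is a lane-based pawn that steps sideways between lanes on Left and Right input.
; On BeginPlay it reads lane count and width from the level manager and sets its starting middle lane.
; Timelines lerp its Y from the current location toward the target, updating the lane index when finished.
; A Moving flag blocks overlapping moves, and edge checks keep it within the outer lanes.
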(event EventBeginPlay
  (CallFunction|Init))

(event Input|ActionEvents|InputActionLeft
  (params (Key :type Key%20Structure :default "None"))
  (bind _returnvalue (Transformation|GetActorLocation))
  (:Pressed
    ;[1 1 1] Pressed Left whilst in Left most lane
    (if (not (<= (Variables|Default|GetCurrentLane) 1))
      (if (not (Variables|Default|GetbMoving))
        (Variables|Default|SetbMoving true)
        (Variables|Default|SetTargetPosition (- (.y (Transformation|GetActorLocation)) (Variables|Default|GetLaneWidth)))
        (bind _move (Timeline|MoveLeft PlayFromStart)
          (:Update
            (Transformation|SetActorLocation (Math|Vector|MakeVector (.x _returnvalue) (Math|Float|Lerp (.y _returnvalue) (Variables|Default|GetTargetPosition) _move) (.z _returnvalue)) false false))
          (:Finished
            (Variables|Default|SetbMoving false)
            (Math|Integer|DecrementInt (Variables|Default|GetCurrentLane))))))))

(event Input|ActionEvents|InputActionRight
  (params (Key :type Key%20Structure :default "None"))
  (bind _returnvalue (Transformation|GetActorLocation))
  (:Pressed
    ;[1 1 1] Pressed Right whilst in the Right most lane
    (if (not (== (Variables|Default|GetCurrentLane) (Variables|/Game/Gameplay/Blueprints/BP_LevelManager.BP_LevelManager_C|GetNumberOfLanes (Variables|Default|GetLevelManagerRef))))
      (if (not (Variables|Default|GetbMoving))
        (Variables|Default|SetbMoving true)
        (Variables|Default|SetTargetPosition (+ (.y (Transformation|GetActorLocation)) (Variables|Default|GetLaneWidth)))
        (bind _move (Timeline|MoveRight PlayFromStart)
          (:Update
            (Transformation|SetActorLocation (Math|Vector|MakeVector (.x _returnvalue) (Math|Float|Lerp (.y _returnvalue) (Variables|Default|GetTargetPosition) _move) (.z _returnvalue)) false false))
          (:Finished
            (Variables|Default|SetbMoving false)
            (Math|Integer|IncrementInt (Variables|Default|GetCurrentLane))))))))

(fn ConstructionScript)

(fn Init
  (bind _output (Utilities|GetLevelManager)
    (:Is%20Valid
      (Variables|Default|SetLevelManagerRef _output)
      (Variables|Default|SetCurrentLane (+ (/ (Variables|/Game/Gameplay/Blueprints/BP_LevelManager.BP_LevelManager_C|GetNumberOfLanes (Variables|Default|GetLevelManagerRef)) 2) 1))
      (Variables|Default|SetLaneWidth (Variables|/Game/Gameplay/Blueprints/BP_LevelManager.BP_LevelManager_C|GetLaneWidth (Variables|Default|GetLevelManagerRef))))
    (:Is%20Not%20Valid
      (Development|PrintString "No Level Manager Found"))))