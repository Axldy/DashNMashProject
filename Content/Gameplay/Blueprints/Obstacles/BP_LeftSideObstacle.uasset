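; Left-side obstacle that dresses itself as a random village or farm prop.
; The construction script destroys its child actor and skeletal mesh, then picks one of fifteen static meshes.
; Zombie, Skeleton and Ghoul events set type flags and idle animations on that skeletal mesh.
; Both overlap events are empty; the hit logic for invincibility, scored kills, attack animations and game over is disconnected and never runs.
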(event OnComponentBeginOverlap(StaticMesh)
  (params (OverlappedComponent :type Primitive%20Component%20Object%20Reference) (OtherActor :type Actor%20Object%20Reference) (OtherComp :type Primitive%20Component%20Object%20Reference) (OtherBodyIndex :type Integer) (bFromSweep :type Boolean) (SweepResult :type Hit%20Result%20Structure%20%28by%20ref%29)))

(event OnComponentBeginOverlap(SkeletalMesh)
  (params (OverlappedComponent :type Primitive%20Component%20Object%20Reference) (OtherActor :type Actor%20Object%20Reference) (OtherComp :type Primitive%20Component%20Object%20Reference) (OtherBodyIndex :type Integer) (bFromSweep :type Boolean) (SweepResult :type Hit%20Result%20Structure%20%28by%20ref%29)))

(event Custom|ZombieSpawned
  (Components|Animation|PlayAnimation (Variables|Default|GetSkeletalMesh) "/Game/UndeadPack/Zombie/Animations/Anim_Idle.Anim_Idle" true)
  (Variables|Default|SetZombie? true))

(event Custom|GhoulSpawned
  (Components|Animation|PlayAnimation (Variables|Default|GetSkeletalMesh) "/Game/UndeadPack/Ghoul/Animations/Anim_Idle.Anim_Idle" true)
  (Variables|Default|SetGhoul? true))

(event Custom|SkeletonSpawned
  (Components|Animation|PlayAnimation (Variables|Default|GetSkeletalMesh) "/Game/UndeadPack/SkeletonEnemy/Animations/Anim_Idle.Anim_Idle" true)
  (Variables|Default|SetSkeleton? true))

(event Custom|PopUp
  (params (ScorePoints :type Float%20%28single-precision%29))
  (Default|PlayHitAnimation (Variables|/Game/Gameplay/Blueprints/Game/BP_GameModeBase.BP_GameModeBase_C|GetHUD (Variables|Default|GetAs%20BP%20Game%20Mode%20Base)) ScorePoints))

(event EventBeginPlay
  (Variables|Default|SetAs%20BP%20Game%20Mode%20Base (.AsBP%20Game%20Mode%20Base (Utilities|Casting|CastToBP_GameModeBase (Game|GetGameMode)))))

(fn ConstructionScript
  (Components|DestroyComponent (Variables|Default|GetChildActor))
  (Components|DestroyComponent (Variables|Default|GetSkeletalMesh))
  (switch int (Math|Random|RandomIntegerinRange 0 14)
    (:0
      (Components|StaticMesh|SetStaticMesh (Variables|Default|GetStaticMesh) "/Game/Gameplay/Assets/Meshes/SideMeshes/SM_ObstacleSideLeft_House.SM_ObstacleSideLeft_House"))
    (:1
      (Components|StaticMesh|SetStaticMesh (Variables|Default|GetStaticMesh) "/Game/Gameplay/Assets/Meshes/SideMeshes/SM_ObstacleSideLeft_CabbagePatch.SM_ObstacleSideLeft_CabbagePatch"))
    (:2
      (Components|StaticMesh|SetStaticMesh (Variables|Default|GetStaticMesh) "/Game/Gameplay/Assets/Meshes/SideMeshes/SM_ObstacleSideLeft_CarrotPatch.SM_ObstacleSideLeft_CarrotPatch"))
    (:3
      (Components|StaticMesh|SetStaticMesh (Variables|Default|GetStaticMesh) "/Game/Gameplay/Assets/Meshes/SideMeshes/SM_ObstacleSideLeft_CornPatch.SM_ObstacleSideLeft_CornPatch"))
    (:4
      (Components|StaticMesh|SetStaticMesh (Variables|Default|GetStaticMesh) "/Game/Gameplay/Assets/Meshes/SideMeshes/SM_ObstacleSideLeft_Lighthouse.SM_ObstacleSideLeft_Lighthouse"))
    (:5
      (Components|StaticMesh|SetStaticMesh (Variables|Default|GetStaticMesh) "/Game/Gameplay/Assets/Meshes/SideMeshes/SM_ObstacleSideLeft_Mill.SM_ObstacleSideLeft_Mill"))
    (:6
      (Components|StaticMesh|SetStaticMesh (Variables|Default|GetStaticMesh) "/Game/Gameplay/Assets/Meshes/SideMeshes/SM_ObstacleSideLeft_OnionPatch.SM_ObstacleSideLeft_OnionPatch"))
    (:7
      (Components|StaticMesh|SetStaticMesh (Variables|Default|GetStaticMesh) "/Game/Gameplay/Assets/Meshes/SideMeshes/SM_ObstacleSideLeft_PumpkinPatch.SM_ObstacleSideLeft_PumpkinPatch"))
    (:8
      (Components|StaticMesh|SetStaticMesh (Variables|Default|GetStaticMesh) "/Game/Gameplay/Assets/Meshes/SideMeshes/SM_ObstacleSideLeft_Barn.SM_ObstacleSideLeft_Barn"))
    (:9
      (Components|StaticMesh|SetStaticMesh (Variables|Default|GetStaticMesh) "/Game/Gameplay/Assets/Meshes/SideMeshes/SM_ObstacleSideLeft_House2.SM_ObstacleSideLeft_House2"))
    (:10
      (Components|StaticMesh|SetStaticMesh (Variables|Default|GetStaticMesh) "/Game/Gameplay/Assets/Meshes/SideMeshes/SM_ObstacleSideLeft_House3.SM_ObstacleSideLeft_House3"))
    (:11
      (Components|StaticMesh|SetStaticMesh (Variables|Default|GetStaticMesh) "/Game/Gameplay/Assets/Meshes/SideMeshes/SM_ObstacleSideLeft_Market.SM_ObstacleSideLeft_Market"))
    (:12
      (Components|StaticMesh|SetStaticMesh (Variables|Default|GetStaticMesh) "/Game/Gameplay/Assets/Meshes/SideMeshes/SM_ObstacleSideLeft_Stalls.SM_ObstacleSideLeft_Stalls"))
    (:13
      (Components|StaticMesh|SetStaticMesh (Variables|Default|GetStaticMesh) "/Game/Gameplay/Assets/Meshes/SideMeshes/SM_ObstacleSideLeft_Stairs.SM_ObstacleSideLeft_Stairs"))
    (:14
      (Components|StaticMesh|SetStaticMesh (Variables|Default|GetStaticMesh) "/Game/Gameplay/Assets/Meshes/SideMeshes/SM_ObstacleSideLeft_Stumps.SM_ObstacleSideLeft_Stumps"))))

(fn ReturnParent
  (return (Variables|Default|GetParentRef)))

(fn SetParent
  (params (Parent :type BP%20Spawner%20Base%20Object%20Reference))
  (Variables|Default|SetParentRef Parent)
  (return false))