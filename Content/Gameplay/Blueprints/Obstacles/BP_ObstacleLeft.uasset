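; Randomized left-side obstacle that builds itself as a static prop, an enemy or a pickup.
; The Construction Script rolls weighted content and destroys unused components: props (some with airborne coins), zombie, skeleton or ghoul, or coins and power-ups.
; Attacking or invincible players kill enemies for type-based score and kill points, and invincibility also smashes props.
; Any other overlap calls HitObstacle and LevelManager GameOver, with enemies playing random attack animations.
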(event OnComponentBeginOverlap(StaticMesh)
  (params (OverlappedComponent :type Primitive%20Component%20Object%20Reference) (OtherActor :type Actor%20Object%20Reference) (OtherComp :type Primitive%20Component%20Object%20Reference) (OtherBodyIndex :type Integer) (bFromSweep :type Boolean) (SweepResult :type Hit%20Result%20Structure%20%28by%20ref%29))
  (bind (_levelmanager _levelmanagerfound) (CallFunction|GetLevelManager))
  (bind _asbp_pawn_base (Utilities|Casting|CastToBP_PawnBase OtherActor))
  (if (Variables|/Game/Gameplay/Blueprints/Character/BP_PawnBase.BP_PawnBase_C|GetInvincibilityOn? _asbp_pawn_base)
    (Effects|SpawnEmitteratLocation "/Game/FXVarietyPack/Particles/P_ky_ThunderBallHit.P_ky_ThunderBallHit" (Transformation|GetWorldLocation (Variables|Default|GetStaticMesh)) "0, 0, 0" "0.500000,0.500000,0.500000")
    (Audio|PlaySound2D "/Game/Sounds/SFX/HeavyHit_Cue.HeavyHit_Cue" 1.0 1.0 0.0 0 0)
    (Components|DestroyComponent (Variables|Default|GetStaticMesh))
    (else
      (Default|HitObstacle _asbp_pawn_base)
      (if _levelmanagerfound
        (Default|GameOver _levelmanager)))))

(event OnComponentBeginOverlap(SkeletalMesh)
  (params (OverlappedComponent :type Primitive%20Component%20Object%20Reference) (OtherActor :type Actor%20Object%20Reference) (OtherComp :type Primitive%20Component%20Object%20Reference) (OtherBodyIndex :type Integer) (bFromSweep :type Boolean) (SweepResult :type Hit%20Result%20Structure%20%28by%20ref%29))
  (bind (_levelmanager _levelmanagerfound) (CallFunction|GetLevelManager))
  (bind _as_bp_game_mode_base (Variables|Default|GetAs%20BP%20Game%20Mode%20Base))
  (bind _as_bp_game_mode_base_2 (Variables|Default|GetAs%20BP%20Game%20Mode%20Base))
  (bind _as_bp_game_mode_base_3 (Variables|Default|GetAs%20BP%20Game%20Mode%20Base))
  (bind _skeletalmesh (Variables|Default|GetSkeletalMesh))
  (bind _skeletalmesh_2 (Variables|Default|GetSkeletalMesh))
  (bind _skeletalmesh_3 (Variables|Default|GetSkeletalMesh))
  (bind _as_bp_game_mode_base_4 (Variables|Default|GetAs%20BP%20Game%20Mode%20Base))
  (bind _as_bp_game_mode_base_5 (Variables|Default|GetAs%20BP%20Game%20Mode%20Base))
  (bind _as_bp_game_mode_base_6 (Variables|Default|GetAs%20BP%20Game%20Mode%20Base))
  (bind _asbp_pawn_base (Utilities|Casting|CastToBP_PawnBase OtherActor))
  (if (Variables|/Game/Gameplay/Blueprints/Character/BP_PawnBase.BP_PawnBase_C|GetInvincibilityOn? _asbp_pawn_base)
    (if (Variables|Default|GetZombie?)
      (Default|HitEnemy (Variables|/Game/Gameplay/Blueprints/Game/BP_GameModeBase.BP_GameModeBase_C|GetAs%20BP%20Pawn%20Base (Variables|Default|GetAs%20BP%20Game%20Mode%20Base)) "Zombie")
      (CallFunction|PopUp 1e+02)
      (Default|AddtoScore _as_bp_game_mode_base_3 1e+02)
      (Default|AddKillPoints _as_bp_game_mode_base_3)
      (Effects|SpawnEmitteratLocation "/Game/FXVarietyPack/Particles/P_ky_ThunderBallHit.P_ky_ThunderBallHit" (Transformation|GetWorldLocation (Variables|Default|GetSkeletalMesh)) "0, 0, 0" "0.500000,0.500000,0.500000" :!label _label)
      (Actor|DestroyActor)
      (elif (Variables|Default|GetSkeleton?)
        (Default|HitEnemy (Variables|/Game/Gameplay/Blueprints/Game/BP_GameModeBase.BP_GameModeBase_C|GetAs%20BP%20Pawn%20Base (Variables|Default|GetAs%20BP%20Game%20Mode%20Base)) "Skeleton")
        (CallFunction|PopUp 2.5e+02)
        (Default|AddtoScore _as_bp_game_mode_base_2 2.5e+02)
        (Default|AddKillPoints _as_bp_game_mode_base_2)
        (goto _label)
        (elif (Variables|Default|GetGhoul?)
          (Default|HitEnemy (Variables|/Game/Gameplay/Blueprints/Game/BP_GameModeBase.BP_GameModeBase_C|GetAs%20BP%20Pawn%20Base (Variables|Default|GetAs%20BP%20Game%20Mode%20Base)) "Ghoul")
          (CallFunction|PopUp 5e+02)
          (Default|AddtoScore _as_bp_game_mode_base 5e+02)
          (Default|AddKillPoints _as_bp_game_mode_base)
          (goto _label))))
    (elif (Variables|/Game/Gameplay/Blueprints/Character/BP_PawnBase.BP_PawnBase_C|GetIsAttacking? _asbp_pawn_base)
      (if (Variables|Default|GetZombie?)
        (Collision|SetCollisionEnabled _skeletalmesh "NoCollision")
        (Components|Animation|PlayAnimation _skeletalmesh "/Game/UndeadPack/Zombie/Animations/Anim_Death.Anim_Death" false)
        (Default|HitEnemy (Variables|/Game/Gameplay/Blueprints/Game/BP_GameModeBase.BP_GameModeBase_C|GetAs%20BP%20Pawn%20Base (Variables|Default|GetAs%20BP%20Game%20Mode%20Base)) "Zombie")
        (CallFunction|PopUp 1e+02)
        (Default|AddtoScore _as_bp_game_mode_base_6 1e+02)
        (Default|AddKillPoints _as_bp_game_mode_base_6)
        (Effects|SpawnEmitteratLocation "/Game/FXVarietyPack/Particles/P_ky_lightning2.P_ky_lightning2" (Transformation|GetWorldLocation (Variables|Default|GetSkeletalMesh)) :!label _label_2)
        (Utilities|FlowControl|Delay 1.0)
        (Collision|SetCollisionEnabled (Variables|Default|GetSkeletalMesh) "QueryOnly")
        (elif (Variables|Default|GetSkeleton?)
          (Collision|SetCollisionEnabled _skeletalmesh_2 "NoCollision")
          (Components|Animation|PlayAnimation _skeletalmesh_2 "/Game/UndeadPack/SkeletonEnemy/Animations/Anim_Death.Anim_Death" false)
          (Default|HitEnemy (Variables|/Game/Gameplay/Blueprints/Game/BP_GameModeBase.BP_GameModeBase_C|GetAs%20BP%20Pawn%20Base (Variables|Default|GetAs%20BP%20Game%20Mode%20Base)) "Skeleton")
          (CallFunction|PopUp 2.5e+02)
          (Default|AddtoScore _as_bp_game_mode_base_5 2.5e+02)
          (Default|AddKillPoints _as_bp_game_mode_base_5)
          (goto _label_2)
          (elif (Variables|Default|GetGhoul?)
            (Collision|SetCollisionEnabled _skeletalmesh_3 "NoCollision")
            (Components|Animation|PlayAnimation _skeletalmesh_3 "/Game/UndeadPack/Ghoul/Animations/Anim_Death.Anim_Death" false)
            (Default|HitEnemy (Variables|/Game/Gameplay/Blueprints/Game/BP_GameModeBase.BP_GameModeBase_C|GetAs%20BP%20Pawn%20Base (Variables|Default|GetAs%20BP%20Game%20Mode%20Base)) "Ghoul")
            (CallFunction|PopUp 5e+02)
            (Default|AddtoScore _as_bp_game_mode_base_4 5e+02)
            (Default|AddKillPoints _as_bp_game_mode_base_4)
            (goto _label_2))))
      (else
        (Utilities|FlowControl|DoOnce false
          (:Completed
            (Default|HitObstacle _asbp_pawn_base)
            (if _levelmanagerfound
              (Default|GameOver _levelmanager)
              (if (Variables|Default|GetZombie?)
                (switch int (Math|Random|RandomIntegerinRange 0 1)
                  (:0
                    (Components|Animation|PlayAnimation (Variables|Default|GetSkeletalMesh) "/Game/UndeadPack/Zombie/Animations/Anim_Attack1.Anim_Attack1" false)
                    (Utilities|FlowControl|Delay 2.47))
                  (:1
                    (Components|Animation|PlayAnimation (Variables|Default|GetSkeletalMesh) "/Game/UndeadPack/Zombie/Animations/Anim_Attack2.Anim_Attack2" false)
                    (Utilities|FlowControl|Delay 1.97)))
                (Components|Animation|PlayAnimation (Variables|Default|GetSkeletalMesh) "/Game/UndeadPack/Zombie/Animations/Anim_Idle.Anim_Idle" true)
                (elif (Variables|Default|GetSkeleton?)
                  (switch int (Math|Random|RandomIntegerinRange 0 1)
                    (:0
                      (Components|Animation|PlayAnimation (Variables|Default|GetSkeletalMesh) "/Game/UndeadPack/SkeletonEnemy/Animations/Anim_Attack_1.Anim_Attack_1" false)
                      (Utilities|FlowControl|Delay 1.67))
                    (:1
                      (Components|Animation|PlayAnimation (Variables|Default|GetSkeletalMesh) "/Game/UndeadPack/SkeletonEnemy/Animations/Anim_Attack_2.Anim_Attack_2" false)
                      (Utilities|FlowControl|Delay 1.5)))
                  (Components|Animation|PlayAnimation (Variables|Default|GetSkeletalMesh) "/Game/UndeadPack/SkeletonEnemy/Animations/Anim_Idle.Anim_Idle" true)
                  (elif (Variables|Default|GetGhoul?)
                    (switch int (Math|Random|RandomIntegerinRange 0 1)
                      (:0
                        (Components|Animation|PlayAnimation (Variables|Default|GetSkeletalMesh) "/Game/UndeadPack/Ghoul/Animations/Anim_Attack_Left.Anim_Attack_Left" false)
                        (Utilities|FlowControl|Delay 1.17))
                      (:1
                        (Components|Animation|PlayAnimation (Variables|Default|GetSkeletalMesh) "/Game/UndeadPack/Ghoul/Animations/Anim_Attack_Right.Anim_Attack_Right" false)
                        (Utilities|FlowControl|Delay 1.17)))
                    (Components|Animation|PlayAnimation (Variables|Default|GetSkeletalMesh) "/Game/UndeadPack/Ghoul/Animations/Anim_Idle.Anim_Idle" true)))))))))))

(event Custom|ZombieSpawned
  (Components|Animation|PlayAnimation (Variables|Default|GetSkeletalMesh) "/Game/UndeadPack/Zombie/Animations/Anim_Idle.Anim_Idle" true)
  (Variables|Default|SetZombie? true))

(event Custom|GhoulSpawned
  (Components|Animation|PlayAnimation (Variables|Default|GetSkeletalMesh) "/Game/UndeadPack/Ghoul/Animations/Anim_Idle.Anim_Idle" true)
  (Variables|Default|SetGhoul? true))

(event Custom|SkeletonSpawned
  (Components|Animation|PlayAnimation (Variables|Default|GetSkeletalMesh) "/Game/UndeadPack/SkeletonEnemy/Animations/Anim_Idle.Anim_Idle" true)
  (Variables|Default|SetSkeleton? true))

(event Custom|PopUp
  (params (ScorePoints :type Float%20%28single-precision%29))
  (Default|PlayHitAnimation (Variables|/Game/Gameplay/Blueprints/Game/BP_GameModeBase.BP_GameModeBase_C|GetHUD (Variables|Default|GetAs%20BP%20Game%20Mode%20Base)) ScorePoints))

(event EventBeginPlay
  (Variables|Default|SetAs%20BP%20Game%20Mode%20Base (.AsBP%20Game%20Mode%20Base (Utilities|Casting|CastToBP_GameModeBase (Game|GetGameMode)))))

(fn ConstructionScript
  (switch int (Math|Random|RandomIntegerinRange 0 9)
    (:0
      (Components|DestroyComponent (Variables|Default|GetSkeletalMesh) :!label _label)
      (switch int (Math|Random|RandomIntegerinRange 0 29)
        (:0
          (switch int (Math|Random|RandomIntegerinRange 0 3)
            (:0
              (Components|DestroyComponent (Variables|Default|GetChildActor) :!label _label_2))
            (:1
              (goto _label_2))
            (:2
              (ChildActorComponent|SetChildActorClass (Variables|Default|GetChildActor) "/Game/Gameplay/Blueprints/Pickups/BP_5_Coins_Air.BP_5_Coins_Air_C"))
            (:3
              (ChildActorComponent|SetChildActorClass (Variables|Default|GetChildActor) "/Game/Gameplay/Blueprints/Pickups/BP_7_Coins_Air.BP_7_Coins_Air_C")))
          (Components|StaticMesh|SetStaticMesh (Variables|Default|GetStaticMesh) "/Game/GreenwoodFantasyVillage/Meshes/SM_TreeStumpB.SM_TreeStumpB")
          (Transformation|SetWorldScale3D (Variables|Default|GetStaticMesh) (Math|Vector|MakeVector 1.0 1.0 1.0) :!label _label_3)
          (Transformation|SetWorldRotation (Variables|Default|GetStaticMesh) (Math|Rotator|MakeRotator 0.0 0.0 (Math|Random|RandomFloatinRange 0.0 3.6e+02)) false false :!label _label_4))
        (:1
          (Components|DestroyComponent (Variables|Default|GetChildActor))
          (Components|StaticMesh|SetStaticMesh (Variables|Default|GetStaticMesh) "/Game/GreenwoodFantasyVillage/Meshes/SM_TreeStumpA.SM_TreeStumpA")
          (goto _label_3))
        (:2
          (Components|DestroyComponent (Variables|Default|GetChildActor))
          (Components|StaticMesh|SetStaticMesh (Variables|Default|GetStaticMesh) "/Game/GreenwoodFantasyVillage/Meshes/SM_Tree_A.SM_Tree_A")
          (Transformation|SetWorldScale3D (Variables|Default|GetStaticMesh) (Math|Vector|MakeVector 0.75 0.75 0.75) :!label _label_5)
          (goto _label_4))
        (:3
          (Components|DestroyComponent (Variables|Default|GetChildActor))
          (Components|StaticMesh|SetStaticMesh (Variables|Default|GetStaticMesh) "/Game/GreenwoodFantasyVillage/Meshes/SM_Tree_B.SM_Tree_B")
          (goto _label_5))
        (:4
          (Components|DestroyComponent (Variables|Default|GetChildActor))
          (Components|StaticMesh|SetStaticMesh (Variables|Default|GetStaticMesh) "/Game/GreenwoodFantasyVillage/Meshes/SM_Tree_C.SM_Tree_C")
          (goto _label_5))
        (:5
          (Components|DestroyComponent (Variables|Default|GetChildActor))
          (Components|StaticMesh|SetStaticMesh (Variables|Default|GetStaticMesh) "/Game/GreenwoodFantasyVillage/Meshes/SM_Tree_D.SM_Tree_D")
          (goto _label_5))
        (:6
          (Components|DestroyComponent (Variables|Default|GetChildActor))
          (Components|StaticMesh|SetStaticMesh (Variables|Default|GetStaticMesh) "/Game/GreenwoodFantasyVillage/Meshes/SM_ShopA.SM_ShopA")
          (Transformation|SetWorldScale3D (Variables|Default|GetStaticMesh) (Math|Vector|MakeVector 1.0 1.0 1.0) :!label _label_6)
          (Transformation|SetWorldRotation (Variables|Default|GetStaticMesh) (Math|Rotator|MakeRotator 0.0 0.0 9e+01) false false))
        (:7
          (Components|DestroyComponent (Variables|Default|GetChildActor))
          (Components|StaticMesh|SetStaticMesh (Variables|Default|GetStaticMesh) "/Game/GreenwoodFantasyVillage/Meshes/SM_ShopB.SM_ShopB")
          (goto _label_6))
        (:8
          (Components|DestroyComponent (Variables|Default|GetChildActor))
          (Components|StaticMesh|SetStaticMesh (Variables|Default|GetStaticMesh) "/Game/GreenwoodFantasyVillage/Meshes/SM_ShopC.SM_ShopC")
          (goto _label_6))
        (:9
          (Components|DestroyComponent (Variables|Default|GetChildActor))
          (Components|StaticMesh|SetStaticMesh (Variables|Default|GetStaticMesh) "/Game/GreenwoodFantasyVillage/Meshes/SM_Well.SM_Well")
          (goto _label_6))
        (:10
          (Components|DestroyComponent (Variables|Default|GetChildActor))
          (Components|StaticMesh|SetStaticMesh (Variables|Default|GetStaticMesh) "/Game/GreenwoodFantasyVillage/Meshes/SM_WaymarkA.SM_WaymarkA")
          (Transformation|SetWorldScale3D (Variables|Default|GetStaticMesh) (Math|Vector|MakeVector 1.0 1.0 1.0) :!label _label_7)
          (Transformation|SetWorldRotation (Variables|Default|GetStaticMesh) (Math|Rotator|MakeRotator 0.0 0.0 (Math|Random|RandomFloatinRange 45.0 135.0)) false false))
        (:11
          (Components|DestroyComponent (Variables|Default|GetChildActor))
          (Components|StaticMesh|SetStaticMesh (Variables|Default|GetStaticMesh) "/Game/GreenwoodFantasyVillage/Meshes/SM_WaymarkB.SM_WaymarkB")
          (goto _label_7))
        (:12
          (Components|DestroyComponent (Variables|Default|GetChildActor))
          (Components|StaticMesh|SetStaticMesh (Variables|Default|GetStaticMesh) "/Game/GreenwoodFantasyVillage/Meshes/SM_WaymarkC.SM_WaymarkC")
          (goto _label_7))
        (:13
          (Components|DestroyComponent (Variables|Default|GetChildActor))
          (Components|StaticMesh|SetStaticMesh (Variables|Default|GetStaticMesh) "/Game/GreenwoodFantasyVillage/Meshes/SM_Pumpkin.SM_Pumpkin")
          (Transformation|SetWorldScale3D (Variables|Default|GetStaticMesh) (Math|Conversions|ToVector(Float) (Math|Random|RandomFloatinRange 1.0 1.75)) :!label _label_8)
          (Transformation|SetWorldRotation (Variables|Default|GetStaticMesh) (Math|Rotator|MakeRotator 0.0 0.0 (Math|Random|RandomFloatinRange 0.0 3.6e+02)) false false))
        (:14
          (Components|DestroyComponent (Variables|Default|GetChildActor))
          (Components|StaticMesh|SetStaticMesh (Variables|Default|GetStaticMesh) "/Game/GreenwoodFantasyVillage/Meshes/SM_Crate.SM_Crate")
          (goto _label_8))
        (:15
          (Components|DestroyComponent (Variables|Default|GetChildActor))
          (Components|StaticMesh|SetStaticMesh (Variables|Default|GetStaticMesh) "/Game/GreenwoodFantasyVillage/Meshes/SM_LightStand.SM_LightStand")
          (Transformation|SetWorldScale3D (Variables|Default|GetStaticMesh) (Math|Vector|MakeVector 2.0 2.0 2.0))
          (Transformation|SetWorldRotation (Variables|Default|GetStaticMesh) (Math|Rotator|MakeRotator 0.0 0.0 0.0) false false))
        (:16
          (switch int (Math|Random|RandomIntegerinRange 0 3)
            (:0
              (Components|DestroyComponent (Variables|Default|GetChildActor) :!label _label_9))
            (:1
              (goto _label_9))
            (:2
              (ChildActorComponent|SetChildActorClass (Variables|Default|GetChildActor) "/Game/Gameplay/Blueprints/Pickups/BP_5_Coins_Air.BP_5_Coins_Air_C"))
            (:3
              (ChildActorComponent|SetChildActorClass (Variables|Default|GetChildActor) "/Game/Gameplay/Blueprints/Pickups/BP_7_Coins_Air.BP_7_Coins_Air_C")))
          (Components|StaticMesh|SetStaticMesh (Variables|Default|GetStaticMesh) "/Game/GreenwoodFantasyVillage/Meshes/SM_Barrel.SM_Barrel")
          (Transformation|SetWorldScale3D (Variables|Default|GetStaticMesh) (Math|Vector|MakeVector 1.5 1.5 1.5) :!label _label_10)
          (Transformation|SetWorldRotation (Variables|Default|GetStaticMesh) (Math|Rotator|MakeRotator 0.0 0.0 (Math|Random|RandomFloatinRange 0.0 3.6e+02)) false false))
        (:17
          (switch int (Math|Random|RandomIntegerinRange 0 3)
            (:0
              (Components|DestroyComponent (Variables|Default|GetChildActor) :!label _label_11))
            (:1
              (goto _label_11))
            (:2
              (ChildActorComponent|SetChildActorClass (Variables|Default|GetChildActor) "/Game/Gameplay/Blueprints/Pickups/BP_5_Coins_Air.BP_5_Coins_Air_C"))
            (:3
              (ChildActorComponent|SetChildActorClass (Variables|Default|GetChildActor) "/Game/Gameplay/Blueprints/Pickups/BP_7_Coins_Air.BP_7_Coins_Air_C")))
          (Components|StaticMesh|SetStaticMesh (Variables|Default|GetStaticMesh) "/Game/GreenwoodFantasyVillage/Meshes/SM_BarrelGrain.SM_BarrelGrain")
          (goto _label_10))
        (:18
          (Components|DestroyComponent (Variables|Default|GetChildActor))
          (Components|StaticMesh|SetStaticMesh (Variables|Default|GetStaticMesh) "/Game/GreenwoodFantasyVillage/Meshes/SM_BonfireAessembled.SM_BonfireAessembled")
          (goto _label_10))
        (:19
          (switch int (Math|Random|RandomIntegerinRange 0 3)
            (:0
              (Components|DestroyComponent (Variables|Default|GetChildActor) :!label _label_12))
            (:1
              (goto _label_12))
            (:2
              (ChildActorComponent|SetChildActorClass (Variables|Default|GetChildActor) "/Game/Gameplay/Blueprints/Pickups/BP_5_Coins_Air.BP_5_Coins_Air_C"))
            (:3
              (ChildActorComponent|SetChildActorClass (Variables|Default|GetChildActor) "/Game/Gameplay/Blueprints/Pickups/BP_7_Coins_Air.BP_7_Coins_Air_C")))
          (Components|StaticMesh|SetStaticMesh (Variables|Default|GetStaticMesh) "/Game/GreenwoodFantasyVillage/Meshes/SM_Bench.SM_Bench")
          (Transformation|SetWorldScale3D (Variables|Default|GetStaticMesh) (Math|Vector|MakeVector 2.0 2.0 2.0))
          (Transformation|SetWorldRotation (Variables|Default|GetStaticMesh) (Math|Rotator|MakeRotator 0.0 0.0 (Math|Random|RandomFloatinRange 45.0 135.0)) false false :!label _label_13))
        (:20
          (switch int (Math|Random|RandomIntegerinRange 0 3)
            (:0
              (Components|DestroyComponent (Variables|Default|GetChildActor) :!label _label_14))
            (:1
              (goto _label_14))
            (:2
              (ChildActorComponent|SetChildActorClass (Variables|Default|GetChildActor) "/Game/Gameplay/Blueprints/Pickups/BP_5_Coins_Air.BP_5_Coins_Air_C"))
            (:3
              (ChildActorComponent|SetChildActorClass (Variables|Default|GetChildActor) "/Game/Gameplay/Blueprints/Pickups/BP_7_Coins_Air.BP_7_Coins_Air_C")))
          (Components|StaticMesh|SetStaticMesh (Variables|Default|GetStaticMesh) "/Game/GreenwoodFantasyVillage/Meshes/SM_Billboard.SM_Billboard")
          (Transformation|SetWorldScale3D (Variables|Default|GetStaticMesh) (Math|Vector|MakeVector 1.0 1.0 1.0))
          (goto _label_13))
        (:21
          (switch int (Math|Random|RandomIntegerinRange 0 3)
            (:0
              (Components|DestroyComponent (Variables|Default|GetChildActor) :!label _label_15))
            (:1
              (goto _label_15))
            (:2
              (ChildActorComponent|SetChildActorClass (Variables|Default|GetChildActor) "/Game/Gameplay/Blueprints/Pickups/BP_5_Coins_Air.BP_5_Coins_Air_C"))
            (:3
              (ChildActorComponent|SetChildActorClass (Variables|Default|GetChildActor) "/Game/Gameplay/Blueprints/Pickups/BP_7_Coins_Air.BP_7_Coins_Air_C")))
          (Components|StaticMesh|SetStaticMesh (Variables|Default|GetStaticMesh) "/Game/GreenwoodFantasyVillage/Meshes/SM_Boat.SM_Boat")
          (Transformation|SetWorldScale3D (Variables|Default|GetStaticMesh) (Math|Vector|MakeVector 1.0 1.0 1.0))
          (switch int (Math|Random|RandomIntegerinRange 0 1)
            (:0
              (Transformation|SetWorldRotation (Variables|Default|GetStaticMesh) (Math|Rotator|MakeRotator 0.0 0.0 (Math|Random|RandomFloatinRange 165.0 195.0)) false false))
            (:1
              (Transformation|SetWorldRotation (Variables|Default|GetStaticMesh) (Math|Rotator|MakeRotator 0.0 0.0 (Math|Random|RandomFloatinRange -15.0 15.0)) false false))))
        (:22
          (switch int (Math|Random|RandomIntegerinRange 0 3)
            (:0
              (Components|DestroyComponent (Variables|Default|GetChildActor) :!label _label_16))
            (:1
              (goto _label_16))
            (:2
              (ChildActorComponent|SetChildActorClass (Variables|Default|GetChildActor) "/Game/Gameplay/Blueprints/Pickups/BP_5_Coins_Air.BP_5_Coins_Air_C"))
            (:3
              (ChildActorComponent|SetChildActorClass (Variables|Default|GetChildActor) "/Game/Gameplay/Blueprints/Pickups/BP_7_Coins_Air.BP_7_Coins_Air_C")))
          (Components|StaticMesh|SetStaticMesh (Variables|Default|GetStaticMesh) "/Game/GreenwoodFantasyVillage/Meshes/SM_BushBig_A.SM_BushBig_A")
          (Transformation|SetWorldScale3D (Variables|Default|GetStaticMesh) (Math|Vector|MakeVector 0.75 0.75 0.75) :!label _label_17)
          (Transformation|SetWorldRotation (Variables|Default|GetStaticMesh) (Math|Rotator|MakeRotator 0.0 0.0 (Math|Random|RandomFloatinRange 0.0 3.6e+02)) false false))
        (:23
          (switch int (Math|Random|RandomIntegerinRange 0 3)
            (:0
              (Components|DestroyComponent (Variables|Default|GetChildActor) :!label _label_18))
            (:1
              (goto _label_18))
            (:2
              (ChildActorComponent|SetChildActorClass (Variables|Default|GetChildActor) "/Game/Gameplay/Blueprints/Pickups/BP_5_Coins_Air.BP_5_Coins_Air_C"))
            (:3
              (ChildActorComponent|SetChildActorClass (Variables|Default|GetChildActor) "/Game/Gameplay/Blueprints/Pickups/BP_7_Coins_Air.BP_7_Coins_Air_C")))
          (Components|StaticMesh|SetStaticMesh (Variables|Default|GetStaticMesh) "/Game/GreenwoodFantasyVillage/Meshes/SM_BushBig_B.SM_BushBig_B")
          (goto _label_17))
        (:24
          (switch int (Math|Random|RandomIntegerinRange 0 3)
            (:0
              (Components|DestroyComponent (Variables|Default|GetChildActor) :!label _label_19))
            (:1
              (goto _label_19))
            (:2
              (ChildActorComponent|SetChildActorClass (Variables|Default|GetChildActor) "/Game/Gameplay/Blueprints/Pickups/BP_5_Coins_Air.BP_5_Coins_Air_C"))
            (:3
              (ChildActorComponent|SetChildActorClass (Variables|Default|GetChildActor) "/Game/Gameplay/Blueprints/Pickups/BP_7_Coins_Air.BP_7_Coins_Air_C")))
          (Components|StaticMesh|SetStaticMesh (Variables|Default|GetStaticMesh) "/Game/GreenwoodFantasyVillage/Meshes/SM_BushBig_C.SM_BushBig_C")
          (goto _label_17))
        (:25
          (Components|DestroyComponent (Variables|Default|GetChildActor))
          (Components|StaticMesh|SetStaticMesh (Variables|Default|GetStaticMesh) "/Game/GreenwoodFantasyVillage/Meshes/SM_Barn.SM_Barn")
          (Transformation|SetWorldScale3D (Variables|Default|GetStaticMesh) (Math|Vector|MakeVector 0.5 0.5 0.5))
          (Transformation|SetWorldRotation (Variables|Default|GetStaticMesh) (Math|Rotator|MakeRotator 0.0 0.0 9e+01) false false))
        (:26
          (Components|DestroyComponent (Variables|Default|GetChildActor))
          (Components|StaticMesh|SetStaticMesh (Variables|Default|GetStaticMesh) "/Game/GreenwoodFantasyVillage/Meshes/SM_HouseB.SM_HouseB")
          (Transformation|SetWorldScale3D (Variables|Default|GetStaticMesh) (Math|Vector|MakeVector 0.75 0.75 0.75))
          (Transformation|SetWorldRotation (Variables|Default|GetStaticMesh) (Math|Rotator|MakeRotator 0.0 0.0 0.0) false false))
        (:27
          (Components|DestroyComponent (Variables|Default|GetChildActor))
          (Components|StaticMesh|SetStaticMesh (Variables|Default|GetStaticMesh) "/Game/GreenwoodFantasyVillage/Meshes/SM_Mill.SM_Mill")
          (Transformation|SetWorldScale3D (Variables|Default|GetStaticMesh) (Math|Vector|MakeVector 0.75 0.75 0.5))
          (Transformation|SetWorldRotation (Variables|Default|GetStaticMesh) (Math|Rotator|MakeRotator 0.0 0.0 2.7e+02) false false))
        (:28
          (switch int (Math|Random|RandomIntegerinRange 0 3)
            (:0
              (Components|DestroyComponent (Variables|Default|GetChildActor) :!label _label_20))
            (:1
              (goto _label_20))
            (:2
              (ChildActorComponent|SetChildActorClass (Variables|Default|GetChildActor) "/Game/Gameplay/Blueprints/Pickups/BP_5_Coins_Air.BP_5_Coins_Air_C"))
            (:3
              (ChildActorComponent|SetChildActorClass (Variables|Default|GetChildActor) "/Game/Gameplay/Blueprints/Pickups/BP_7_Coins_Air.BP_7_Coins_Air_C")))
          (Components|StaticMesh|SetStaticMesh (Variables|Default|GetStaticMesh) "/Game/GreenwoodFantasyVillage/Meshes/SM_FenceSmallA_2m.SM_FenceSmallA_2m")
          (Transformation|SetWorldScale3D (Variables|Default|GetStaticMesh) (Math|Vector|MakeVector 1.0 1.0 1.0) :!label _label_21)
          (Transformation|SetWorldRotation (Variables|Default|GetStaticMesh) (Math|Rotator|MakeRotator 0.0 0.0 9e+01) false false))
        (:29
          (switch int (Math|Random|RandomIntegerinRange 0 3)
            (:0
              (Components|DestroyComponent (Variables|Default|GetChildActor) :!label _label_22))
            (:1
              (goto _label_22))
            (:2
              (ChildActorComponent|SetChildActorClass (Variables|Default|GetChildActor) "/Game/Gameplay/Blueprints/Pickups/BP_5_Coins_Air.BP_5_Coins_Air_C"))
            (:3
              (ChildActorComponent|SetChildActorClass (Variables|Default|GetChildActor) "/Game/Gameplay/Blueprints/Pickups/BP_7_Coins_Air.BP_7_Coins_Air_C")))
          (Components|StaticMesh|SetStaticMesh (Variables|Default|GetStaticMesh) "/Game/GreenwoodFantasyVillage/Meshes/SM_FenceSmallB_2m.SM_FenceSmallB_2m")
          (goto _label_21))))
    (:1
      (goto _label))
    (:2
      (goto _label))
    (:3
      (goto _label))
    (:4
      (goto _label))
    (:5
      (goto _label))
    (:6
      (goto _label))
    (:7
      (Components|DestroyComponent (Variables|Default|GetStaticMesh) :!label _label_23)
      (Components|DestroyComponent (Variables|Default|GetChildActor))
      (switch int (Math|Random|RandomIntegerinRange 0 5)
        (:0
          (Class|SkinnedMeshComponent|SetSkeletalMesh (Variables|Default|GetSkeletalMesh) "/Game/UndeadPack/Zombie/Mesh/SK_Zombie.SK_Zombie" true :!label _label_24)
          (Transformation|SetWorldScale3D (Variables|Default|GetSkeletalMesh) (Math|Vector|MakeVector 0.9 0.9 0.9))
          (CallFunction|ZombieSpawned))
        (:1
          (goto _label_24))
        (:2
          (goto _label_24))
        (:3
          (Class|SkinnedMeshComponent|SetSkeletalMesh (Variables|Default|GetSkeletalMesh) "/Game/UndeadPack/SkeletonEnemy/Mesh/SK_Skeleton.SK_Skeleton" true :!label _label_25)
          (Transformation|SetWorldScale3D (Variables|Default|GetSkeletalMesh) (Math|Vector|MakeVector 1.8 1.8 1.8))
          (CallFunction|SkeletonSpawned))
        (:4
          (goto _label_25))
        (:5
          (Class|SkinnedMeshComponent|SetSkeletalMesh (Variables|Default|GetSkeletalMesh) "/Game/UndeadPack/Ghoul/Mesh/SK_Ghoul_Full.SK_Ghoul_Full" true)
          (Transformation|SetWorldScale3D (Variables|Default|GetSkeletalMesh) (Math|Vector|MakeVector 2.0 2.0 2.0))
          (CallFunction|GhoulSpawned))))
    (:8
      (goto _label_23))
    (:9
      (Components|DestroyComponent (Variables|Default|GetSkeletalMesh))
      (Components|DestroyComponent (Variables|Default|GetStaticMesh))
      (switch int (Math|Random|RandomIntegerinRange 0 4)
        (:0
          (switch int (Math|Random|RandomIntegerinRange 0 1)
            (:0
              (ChildActorComponent|SetChildActorClass (Variables|Default|GetChildActor) "/Game/Gameplay/Blueprints/Pickups/BP_PowerUp_CoinMagnet.BP_PowerUp_CoinMagnet_C"))
            (:1
              (ChildActorComponent|SetChildActorClass (Variables|Default|GetChildActor) "/Game/Gameplay/Blueprints/Pickups/BP_PowerUp_Invincible.BP_PowerUp_Invincible_C"))))
        (:1
          (ChildActorComponent|SetChildActorClass (Variables|Default|GetChildActor) "/Game/Gameplay/Blueprints/Pickups/BP_5_Coins.BP_5_Coins_C" :!label _label_26))
        (:2
          (goto _label_26))
        (:3
          (goto _label_26))
        (:4
          (goto _label_26))))))

(fn ReturnParent
  (return (Variables|Default|GetParentRef)))

(fn SetParent
  (params (Parent :type BP%20Spawner%20Base%20Object%20Reference))
  (Variables|Default|SetParentRef Parent)
  (return false))