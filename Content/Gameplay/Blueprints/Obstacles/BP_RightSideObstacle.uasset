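; Right-side obstacle actor that dresses itself as random scenery such as houses, crop patches, landmarks or props.
; Its construction script destroys the ChildActor and SkeletalMesh components, then uses nested random switches to pick the static mesh by category and variant.
; Zombie, skeleton and ghoul spawn events set type flags and request idle animation on that skeletal mesh.
; PopUp sends score to the game mode's HUD hit animation, and ParentRef has accessor functions.
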(event Custom|ZombieSpawned
  (Components|Animation|PlayAnimation (Variables|Default|GetSkeletalMesh) "/Game/UndeadPack/Zombie/Animations/Anim_Idle.Anim_Idle" true)
  (Variables|Default|SetZombie? true))

(event Custom|GhoulSpawned
  (Components|Animation|PlayAnimation (Variables|Default|GetSkeletalMesh) "/Game/UndeadPack/Ghoul/Animations/Anim_Idle.Anim_Idle" true)
  (Variables|Default|SetGhoul? true))

(event Custom|SkeletonSpawned
  (Components|Animation|PlayAnimation (Variables|Default|GetSkeletalMesh) "/Game/UndeadPack/SkeletonEnemy/Animations/Anim_Idle.Anim_Idle" true)
  (Variables|Default|SetSkeleton? true))

(event Custom|PopUp
  (params (ScorePoints :type Float%20%28single-precision%29))
  (Default|PlayHitAnimation (Variables|/Game/Gameplay/Blueprints/Game/BP_GameModeBase.BP_GameModeBase_C|GetHUD (Variables|Default|GetAs%20BP%20Game%20Mode%20Base)) ScorePoints))

(event EventBeginPlay
  (Variables|Default|SetAs%20BP%20Game%20Mode%20Base (.AsBP%20Game%20Mode%20Base (Utilities|Casting|CastToBP_GameModeBase (Game|GetGameMode)))))

(fn ConstructionScript
  (Components|DestroyComponent (Variables|Default|GetChildActor))
  (Components|DestroyComponent (Variables|Default|GetSkeletalMesh))
  (switch int (Math|Random|RandomIntegerinRange 0 8)
    (:0
      (switch int (Math|Random|RandomIntegerinRange 0 4)
        (:0
          (Components|StaticMesh|SetStaticMesh (Variables|Default|GetStaticMesh) "/Game/Gameplay/Assets/Meshes/SideMeshes/SM_ObstacleSide_GreenHouse.SM_ObstacleSide_GreenHouse"))
        (:1
          (Components|StaticMesh|SetStaticMesh (Variables|Default|GetStaticMesh) "/Game/Gameplay/Assets/Meshes/SideMeshes/SM_ObstacleSide_GreenHouse2.SM_ObstacleSide_GreenHouse2"))
        (:2
          (Components|StaticMesh|SetStaticMesh (Variables|Default|GetStaticMesh) "/Game/Gameplay/Assets/Meshes/SideMeshes/SM_ObstacleSide_GreenHouse3.SM_ObstacleSide_GreenHouse3"))
        (:3
          (Components|StaticMesh|SetStaticMesh (Variables|Default|GetStaticMesh) "/Game/Gameplay/Assets/Meshes/SideMeshes/SM_ObstacleSide_GreenHouse4.SM_ObstacleSide_GreenHouse4"))
        (:4
          (Components|StaticMesh|SetStaticMesh (Variables|Default|GetStaticMesh) "/Game/Gameplay/Assets/Meshes/SideMeshes/SM_ObstacleSide_GreenHouse5.SM_ObstacleSide_GreenHouse5"))))
    (:1
      (switch int (Math|Random|RandomIntegerinRange 0 4)
        (:0
          (Components|StaticMesh|SetStaticMesh (Variables|Default|GetStaticMesh) "/Game/Gameplay/Assets/Meshes/SideMeshes/SM_ObstacleSide_RedHouse.SM_ObstacleSide_RedHouse"))
        (:1
          (Components|StaticMesh|SetStaticMesh (Variables|Default|GetStaticMesh) "/Game/Gameplay/Assets/Meshes/SideMeshes/SM_ObstacleSide_RedHouse2.SM_ObstacleSide_RedHouse2"))
        (:2
          (Components|StaticMesh|SetStaticMesh (Variables|Default|GetStaticMesh) "/Game/Gameplay/Assets/Meshes/SideMeshes/SM_ObstacleSide_RedHouse3.SM_ObstacleSide_RedHouse3"))
        (:3
          (Components|StaticMesh|SetStaticMesh (Variables|Default|GetStaticMesh) "/Game/Gameplay/Assets/Meshes/SideMeshes/SM_ObstacleSide_RedHouse4.SM_ObstacleSide_RedHouse4"))
        (:4
          (Components|StaticMesh|SetStaticMesh (Variables|Default|GetStaticMesh) "/Game/Gameplay/Assets/Meshes/SideMeshes/SM_ObstacleSide_RedHouse5.SM_ObstacleSide_RedHouse5"))))
    (:2
      (switch int (Math|Random|RandomIntegerinRange 0 4)
        (:0
          (Components|StaticMesh|SetStaticMesh (Variables|Default|GetStaticMesh) "/Game/Gameplay/Assets/Meshes/SideMeshes/SM_ObstacleSide_BlueHouse.SM_ObstacleSide_BlueHouse"))
        (:1
          (Components|StaticMesh|SetStaticMesh (Variables|Default|GetStaticMesh) "/Game/Gameplay/Assets/Meshes/SideMeshes/SM_ObstacleSide_BlueHouse2.SM_ObstacleSide_BlueHouse2"))
        (:2
          (Components|StaticMesh|SetStaticMesh (Variables|Default|GetStaticMesh) "/Game/Gameplay/Assets/Meshes/SideMeshes/SM_ObstacleSide_BlueHouse3.SM_ObstacleSide_BlueHouse3"))
        (:3
          (Components|StaticMesh|SetStaticMesh (Variables|Default|GetStaticMesh) "/Game/Gameplay/Assets/Meshes/SideMeshes/SM_ObstacleSide_BlueHouse4.SM_ObstacleSide_BlueHouse4"))
        (:4
          (Components|StaticMesh|SetStaticMesh (Variables|Default|GetStaticMesh) "/Game/Gameplay/Assets/Meshes/SideMeshes/SM_ObstacleSide_BlueHouse5.SM_ObstacleSide_BlueHouse5"))))
    (:3
      (switch int (Math|Random|RandomIntegerinRange 0 5)
        (:0
          (switch int (Math|Random|RandomIntegerinRange 0 1)
            (:0
              (Components|StaticMesh|SetStaticMesh (Variables|Default|GetStaticMesh) "/Game/Gameplay/Assets/Meshes/SideMeshes/SM_ObstacleSide_CabbagePatch.SM_ObstacleSide_CabbagePatch"))
            (:1
              (Components|StaticMesh|SetStaticMesh (Variables|Default|GetStaticMesh) "/Game/Gameplay/Assets/Meshes/SideMeshes/SM_ObstacleSide_CabbagePatch2.SM_ObstacleSide_CabbagePatch2"))))
        (:1
          (switch int (Math|Random|RandomIntegerinRange 0 1)
            (:0
              (Components|StaticMesh|SetStaticMesh (Variables|Default|GetStaticMesh) "/Game/Gameplay/Assets/Meshes/SideMeshes/SM_ObstacleSide_CarrotPatch.SM_ObstacleSide_CarrotPatch"))
            (:1
              (Components|StaticMesh|SetStaticMesh (Variables|Default|GetStaticMesh) "/Game/Gameplay/Assets/Meshes/SideMeshes/SM_ObstacleSide_CarrotPatch2.SM_ObstacleSide_CarrotPatch2"))))
        (:2
          (Components|StaticMesh|SetStaticMesh (Variables|Default|GetStaticMesh) "/Game/Gameplay/Assets/Meshes/SideMeshes/SM_ObstacleSide_CornPatch.SM_ObstacleSide_CornPatch"))
        (:3
          (switch int (Math|Random|RandomIntegerinRange 0 1)
            (:0
              (Components|StaticMesh|SetStaticMesh (Variables|Default|GetStaticMesh) "/Game/Gameplay/Assets/Meshes/SideMeshes/SM_ObstacleSide_OnionPatch.SM_ObstacleSide_OnionPatch"))
            (:1
              (Components|StaticMesh|SetStaticMesh (Variables|Default|GetStaticMesh) "/Game/Gameplay/Assets/Meshes/SideMeshes/SM_ObstacleSide_OnionPatch2.SM_ObstacleSide_OnionPatch2"))))
        (:4
          (switch int (Math|Random|RandomIntegerinRange 0 1)
            (:0
              (Components|StaticMesh|SetStaticMesh (Variables|Default|GetStaticMesh) "/Game/Gameplay/Assets/Meshes/SideMeshes/SM_ObstacleSide_PumpkinPatch.SM_ObstacleSide_PumpkinPatch"))
            (:1
              (Components|StaticMesh|SetStaticMesh (Variables|Default|GetStaticMesh) "/Game/Gameplay/Assets/Meshes/SideMeshes/SM_ObstacleSide_PumpkinPatch2.SM_ObstacleSide_PumpkinPatch2"))))
        (:5
          (Components|StaticMesh|SetStaticMesh (Variables|Default|GetStaticMesh) "/Game/Gameplay/Assets/Meshes/SideMeshes/SM_ObstacleSide_EmptyPatch.SM_ObstacleSide_EmptyPatch"))))
    (:4
      (switch int (Math|Random|RandomIntegerinRange 0 2)
        (:0
          (Components|StaticMesh|SetStaticMesh (Variables|Default|GetStaticMesh) "/Game/Gameplay/Assets/Meshes/SideMeshes/SM_ObstacleSide_Lighthouse.SM_ObstacleSide_Lighthouse"))
        (:1
          (Components|StaticMesh|SetStaticMesh (Variables|Default|GetStaticMesh) "/Game/Gameplay/Assets/Meshes/SideMeshes/SM_ObstacleSide_Lighthouse2.SM_ObstacleSide_Lighthouse2"))
        (:2
          (Components|StaticMesh|SetStaticMesh (Variables|Default|GetStaticMesh) "/Game/Gameplay/Assets/Meshes/SideMeshes/SM_ObstacleSide_Lighthouse3.SM_ObstacleSide_Lighthouse3"))))
    (:5
      (switch int (Math|Random|RandomIntegerinRange 0 3)
        (:0
          (Components|StaticMesh|SetStaticMesh (Variables|Default|GetStaticMesh) "/Game/Gameplay/Assets/Meshes/SideMeshes/SM_ObstacleSide_Mill.SM_ObstacleSide_Mill"))
        (:1
          (Components|StaticMesh|SetStaticMesh (Variables|Default|GetStaticMesh) "/Game/Gameplay/Assets/Meshes/SideMeshes/SM_ObstacleSide_Mill2.SM_ObstacleSide_Mill2"))
        (:2
          (Components|StaticMesh|SetStaticMesh (Variables|Default|GetStaticMesh) "/Game/Gameplay/Assets/Meshes/SideMeshes/SM_ObstacleSide_Mill3.SM_ObstacleSide_Mill3"))
        (:3
          (Components|StaticMesh|SetStaticMesh (Variables|Default|GetStaticMesh) "/Game/Gameplay/Assets/Meshes/SideMeshes/SM_ObstacleSide_Stairs.SM_ObstacleSide_Stairs"))))
    (:6
      (switch int (Math|Random|RandomIntegerinRange 0 2)
        (:0
          (Components|StaticMesh|SetStaticMesh (Variables|Default|GetStaticMesh) "/Game/Gameplay/Assets/Meshes/SideMeshes/SM_ObstacleSide_Barn.SM_ObstacleSide_Barn"))
        (:1
          (Components|StaticMesh|SetStaticMesh (Variables|Default|GetStaticMesh) "/Game/Gameplay/Assets/Meshes/SideMeshes/SM_ObstacleSide_Market.SM_ObstacleSide_Market"))
        (:2
          (Components|StaticMesh|SetStaticMesh (Variables|Default|GetStaticMesh) "/Game/Gameplay/Assets/Meshes/SideMeshes/SM_ObstacleSide_Stalls.SM_ObstacleSide_Stalls"))))
    (:7
      (switch int (Math|Random|RandomIntegerinRange 0 2)
        (:0
          (Components|StaticMesh|SetStaticMesh (Variables|Default|GetStaticMesh) "/Game/Gameplay/Assets/Meshes/SideMeshes/SM_ObstacleSide_Bushes.SM_ObstacleSide_Bushes"))
        (:1
          (Components|StaticMesh|SetStaticMesh (Variables|Default|GetStaticMesh) "/Game/Gameplay/Assets/Meshes/SideMeshes/SM_ObstacleSide_Bushes2.SM_ObstacleSide_Bushes2"))
        (:2
          (Components|StaticMesh|SetStaticMesh (Variables|Default|GetStaticMesh) "/Game/Gameplay/Assets/Meshes/SideMeshes/SM_ObstacleSide_Bushes3.SM_ObstacleSide_Bushes3"))))
    (:8
      (switch int (Math|Random|RandomIntegerinRange 0 2)
        (:0
          (Components|StaticMesh|SetStaticMesh (Variables|Default|GetStaticMesh) "/Game/Gameplay/Assets/Meshes/SideMeshes/SM_ObstacleSide_CratesAndBarrels.SM_ObstacleSide_CratesAndBarrels"))
        (:1
          (Components|StaticMesh|SetStaticMesh (Variables|Default|GetStaticMesh) "/Game/Gameplay/Assets/Meshes/SideMeshes/SM_ObstacleSide_CratesAndBarrels2.SM_ObstacleSide_CratesAndBarrels2"))
        (:2
          (Components|StaticMesh|SetStaticMesh (Variables|Default|GetStaticMesh) "/Game/Gameplay/Assets/Meshes/SideMeshes/SM_ObstacleSide_Stumps.SM_ObstacleSide_Stumps"))))))

(fn ReturnParent
  (return (Variables|Default|GetParentRef)))

(fn SetParent
  (params (Parent :type BP%20Spawner%20Base%20Object%20Reference))
  (Variables|Default|SetParentRef Parent)
  (return false))