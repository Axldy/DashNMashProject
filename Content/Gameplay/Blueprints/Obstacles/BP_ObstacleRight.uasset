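; Randomized runner obstacle that becomes either a static prop or a Zombie, Skeleton or Ghoul enemy.
; The Construction Script rolls the type, destroys the unused mesh component and randomizes props, usually with per-mesh scale and yaw.
; Props end the game on pawn overlap via the Level Manager.
; Enemies die if the pawn is attacking; otherwise they trigger game over once and play a random attack animation.
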(event OnComponentBeginOverlap(StaticMesh)
  (params (OverlappedComponent :type Primitive%20Component%20Object%20Reference) (OtherActor :type Actor%20Object%20Reference) (OtherComp :type Primitive%20Component%20Object%20Reference) (OtherBodyIndex :type Integer) (bFromSweep :type Boolean) (SweepResult :type Hit%20Result%20Structure%20%28by%20ref%29))
  (bind (_levelmanager _levelmanagerfound) (CallFunction|GetLevelManager))
  (bind _asbp_pawn_base (Utilities|Casting|CastToBP_PawnBase OtherActor))
  (Default|HitObstacle _asbp_pawn_base)
  (if _levelmanagerfound
    (Default|GameOver _levelmanager)))

(event OnComponentBeginOverlap(SkeletalMesh)
  (params (OverlappedComponent :type Primitive%20Component%20Object%20Reference) (OtherActor :type Actor%20Object%20Reference) (OtherComp :type Primitive%20Component%20Object%20Reference) (OtherBodyIndex :type Integer) (bFromSweep :type Boolean) (SweepResult :type Hit%20Result%20Structure%20%28by%20ref%29))
  (bind (_levelmanager _levelmanagerfound) (CallFunction|GetLevelManager))
  (bind _skeletalmesh (Variables|Default|GetSkeletalMesh))
  (bind _skeletalmesh_2 (Variables|Default|GetSkeletalMesh))
  (bind _skeletalmesh_3 (Variables|Default|GetSkeletalMesh))
  (bind _asbp_pawn_base (Utilities|Casting|CastToBP_PawnBase OtherActor))
  (if (Variables|/Game/Gameplay/Blueprints/Character/BP_PawnBase.BP_PawnBase_C|GetIsAttacking? _asbp_pawn_base)
    (if (Variables|Default|GetZombie?)
      (Collision|SetCollisionEnabled _skeletalmesh_2 "NoCollision")
      (Components|Animation|PlayAnimation _skeletalmesh_2 "/Game/UndeadPack/Zombie/Animations/Anim_Death.Anim_Death" false)
      (elif (Variables|Default|GetSkeleton?)
        (Collision|SetCollisionEnabled _skeletalmesh "NoCollision")
        (Components|Animation|PlayAnimation _skeletalmesh "/Game/UndeadPack/SkeletonEnemy/Animations/Anim_Death.Anim_Death" false)
        (elif (Variables|Default|GetGhoul?)
          (Collision|SetCollisionEnabled _skeletalmesh_3 "NoCollision")
          (Components|Animation|PlayAnimation _skeletalmesh_3 "/Game/UndeadPack/Ghoul/Animations/Anim_Death.Anim_Death" false))))
    (else
      (Utilities|FlowControl|DoOnce false
        (:Completed
          (Default|HitObstacle _asbp_pawn_base)
          (if _levelmanagerfound
            (Default|GameOver _levelmanager)
            (if (Variables|Default|GetZombie?)
              (switch int (Math|Random|RandomIntegerinRange 0 1)
                (:0
                  (Components|Animation|PlayAnimation (Variables|Default|GetSkeletalMesh) "/Game/UndeadPack/Zombie/Animations/Anim_Attack1.Anim_Attack1" false)
                  (Utilities|FlowControl|Delay 2.47))
                (:1
                  (Components|Animation|PlayAnimation (Variables|Default|GetSkeletalMesh) "/Game/UndeadPack/Zombie/Animations/Anim_Attack2.Anim_Attack2" false)
                  (Utilities|FlowControl|Delay 1.97)))
              (Components|Animation|PlayAnimation (Variables|Default|GetSkeletalMesh) "/Game/UndeadPack/Zombie/Animations/Anim_Idle.Anim_Idle" true)
              (elif (Variables|Default|GetSkeleton?)
                (switch int (Math|Random|RandomIntegerinRange 0 1)
                  (:0
                    (Components|Animation|PlayAnimation (Variables|Default|GetSkeletalMesh) "/Game/UndeadPack/SkeletonEnemy/Animations/Anim_Attack_1.Anim_Attack_1" false)
                    (Utilities|FlowControl|Delay 1.67))
                  (:1
                    (Components|Animation|PlayAnimation (Variables|Default|GetSkeletalMesh) "/Game/UndeadPack/SkeletonEnemy/Animations/Anim_Attack_2.Anim_Attack_2" false)
                    (Utilities|FlowControl|Delay 1.5)))
                (Components|Animation|PlayAnimation (Variables|Default|GetSkeletalMesh) "/Game/UndeadPack/SkeletonEnemy/Animations/Anim_Idle.Anim_Idle" true)
                (elif (Variables|Default|GetGhoul?)
                  (switch int (Math|Random|RandomIntegerinRange 0 1)
                    (:0
                      (Components|Animation|PlayAnimation (Variables|Default|GetSkeletalMesh) "/Game/UndeadPack/Ghoul/Animations/Anim_Attack_Left.Anim_Attack_Left" false)
                      (Utilities|FlowControl|Delay 1.17))
                    (:1
                      (Components|Animation|PlayAnimation (Variables|Default|GetSkeletalMesh) "/Game/UndeadPack/Ghoul/Animations/Anim_Attack_Right.Anim_Attack_Right" false)
                      (Utilities|FlowControl|Delay 1.17)))
                  (Components|Animation|PlayAnimation (Variables|Default|GetSkeletalMesh) "/Game/UndeadPack/Ghoul/Animations/Anim_Idle.Anim_Idle" true))))))))))

(event Custom|ZombieSpawned
  (Components|Animation|PlayAnimation (Variables|Default|GetSkeletalMesh) "/Game/UndeadPack/Zombie/Animations/Anim_Idle.Anim_Idle" true)
  (Variables|Default|SetZombie? true))

(event Custom|GhoulSpawned
  (Components|Animation|PlayAnimation (Variables|Default|GetSkeletalMesh) "/Game/UndeadPack/Ghoul/Animations/Anim_Idle.Anim_Idle" true)
  (Variables|Default|SetGhoul? true))

(event Custom|SkeletonSpawned
  (Components|Animation|PlayAnimation (Variables|Default|GetSkeletalMesh) "/Game/UndeadPack/SkeletonEnemy/Animations/Anim_Idle.Anim_Idle" true)
  (Variables|Default|SetSkeleton? true))

(fn ConstructionScript
  (switch int (Math|Random|RandomIntegerinRange 0 2)
    (:0
      (Components|DestroyComponent (Variables|Default|GetSkeletalMesh) :!label _label)
      (switch int (Math|Random|RandomIntegerinRange 0 31)
        (:0
          (Components|StaticMesh|SetStaticMesh (Variables|Default|GetStaticMesh) "/Game/GreenwoodFantasyVillage/Meshes/SM_TreeStumpA.SM_TreeStumpA")
          (Transformation|SetWorldScale3D (Variables|Default|GetStaticMesh) (Math|Vector|MakeVector 1.0 1.0 1.0) :!label _label_2)
          (Transformation|SetWorldRotation (Variables|Default|GetStaticMesh) (Math|Rotator|MakeRotator 0.0 0.0 (Math|Random|RandomFloatinRange 0.0 3.6e+02)) false false :!label _label_3))
        (:1
          (Components|StaticMesh|SetStaticMesh (Variables|Default|GetStaticMesh) "/Game/GreenwoodFantasyVillage/Meshes/SM_TreeStumpB.SM_TreeStumpB")
          (goto _label_2))
        (:2
          (Components|StaticMesh|SetStaticMesh (Variables|Default|GetStaticMesh) "/Game/GreenwoodFantasyVillage/Meshes/SM_Tree_A.SM_Tree_A")
          (Transformation|SetWorldScale3D (Variables|Default|GetStaticMesh) (Math|Vector|MakeVector 0.75 0.75 0.75) :!label _label_4)
          (goto _label_3))
        (:3
          (Components|StaticMesh|SetStaticMesh (Variables|Default|GetStaticMesh) "/Game/GreenwoodFantasyVillage/Meshes/SM_Tree_B.SM_Tree_B")
          (goto _label_4))
        (:4
          (Components|StaticMesh|SetStaticMesh (Variables|Default|GetStaticMesh) "/Game/GreenwoodFantasyVillage/Meshes/SM_Tree_C.SM_Tree_C")
          (goto _label_4))
        (:5
          (Components|StaticMesh|SetStaticMesh (Variables|Default|GetStaticMesh) "/Game/GreenwoodFantasyVillage/Meshes/SM_Tree_D.SM_Tree_D")
          (goto _label_4))
        (:6
          (Components|StaticMesh|SetStaticMesh (Variables|Default|GetStaticMesh) "/Game/GreenwoodFantasyVillage/Meshes/SM_ShopA.SM_ShopA")
          (Transformation|SetWorldScale3D (Variables|Default|GetStaticMesh) (Math|Vector|MakeVector 1.0 1.0 1.0) :!label _label_5)
          (Transformation|SetWorldRotation (Variables|Default|GetStaticMesh) (Math|Rotator|MakeRotator 0.0 0.0 2.7e+02) false false))
        (:7
          (Components|StaticMesh|SetStaticMesh (Variables|Default|GetStaticMesh) "/Game/GreenwoodFantasyVillage/Meshes/SM_ShopB.SM_ShopB")
          (goto _label_5))
        (:8
          (Components|StaticMesh|SetStaticMesh (Variables|Default|GetStaticMesh) "/Game/GreenwoodFantasyVillage/Meshes/SM_ShopC.SM_ShopC")
          (goto _label_5))
        (:9
          (Components|StaticMesh|SetStaticMesh (Variables|Default|GetStaticMesh) "/Game/GreenwoodFantasyVillage/Meshes/SM_Well.SM_Well")
          (goto _label_5))
        (:10
          (Components|StaticMesh|SetStaticMesh (Variables|Default|GetStaticMesh) "/Game/GreenwoodFantasyVillage/Meshes/SM_WaymarkA.SM_WaymarkA")
          (Transformation|SetWorldScale3D (Variables|Default|GetStaticMesh) (Math|Vector|MakeVector 1.0 1.0 1.0) :!label _label_6)
          (Transformation|SetWorldRotation (Variables|Default|GetStaticMesh) (Math|Rotator|MakeRotator 0.0 0.0 (Math|Random|RandomFloatinRange 45.0 135.0)) false false))
        (:11
          (Components|StaticMesh|SetStaticMesh (Variables|Default|GetStaticMesh) "/Game/GreenwoodFantasyVillage/Meshes/SM_WaymarkB.SM_WaymarkB")
          (goto _label_6))
        (:12
          (Components|StaticMesh|SetStaticMesh (Variables|Default|GetStaticMesh) "/Game/GreenwoodFantasyVillage/Meshes/SM_WaymarkC.SM_WaymarkC")
          (goto _label_6))
        (:13
          (Components|StaticMesh|SetStaticMesh (Variables|Default|GetStaticMesh) "/Game/GreenwoodFantasyVillage/Meshes/SM_Pumpkin.SM_Pumpkin")
          (Transformation|SetWorldScale3D (Variables|Default|GetStaticMesh) (Math|Conversions|ToVector(Float) (Math|Random|RandomFloatinRange 1.0 1.75)) :!label _label_7)
          (Transformation|SetWorldRotation (Variables|Default|GetStaticMesh) (Math|Rotator|MakeRotator 0.0 0.0 (Math|Random|RandomFloatinRange 0.0 3.6e+02)) false false))
        (:14
          (Components|StaticMesh|SetStaticMesh (Variables|Default|GetStaticMesh) "/Game/GreenwoodFantasyVillage/Meshes/SM_Crate.SM_Crate")
          (goto _label_7))
        (:15
          (Components|StaticMesh|SetStaticMesh (Variables|Default|GetStaticMesh) "/Game/GreenwoodFantasyVillage/Meshes/SM_LightStand.SM_LightStand")
          (Transformation|SetWorldScale3D (Variables|Default|GetStaticMesh) (Math|Vector|MakeVector 2.0 2.0 2.0))
          (Transformation|SetWorldRotation (Variables|Default|GetStaticMesh) (Math|Rotator|MakeRotator 0.0 0.0 0.0) false false))
        (:16
          (Components|StaticMesh|SetStaticMesh (Variables|Default|GetStaticMesh) "/Game/GreenwoodFantasyVillage/Meshes/SM_Barrel.SM_Barrel")
          (Transformation|SetWorldScale3D (Variables|Default|GetStaticMesh) (Math|Vector|MakeVector 1.5 1.5 1.5) :!label _label_8)
          (Transformation|SetWorldRotation (Variables|Default|GetStaticMesh) (Math|Rotator|MakeRotator 0.0 0.0 (Math|Random|RandomFloatinRange 0.0 3.6e+02)) false false))
        (:17
          (Components|StaticMesh|SetStaticMesh (Variables|Default|GetStaticMesh) "/Game/GreenwoodFantasyVillage/Meshes/SM_BarrelGrain.SM_BarrelGrain")
          (goto _label_8))
        (:18
          (Components|StaticMesh|SetStaticMesh (Variables|Default|GetStaticMesh) "/Game/GreenwoodFantasyVillage/Meshes/SM_BonfireAessembled.SM_BonfireAessembled")
          (goto _label_8))
        (:19
          (Components|StaticMesh|SetStaticMesh (Variables|Default|GetStaticMesh) "/Game/GreenwoodFantasyVillage/Meshes/SM_LightColumn.SM_LightColumn")
          (Transformation|SetWorldScale3D (Variables|Default|GetStaticMesh) (Math|Vector|MakeVector 1.0 1.0 1.0))
          (Transformation|SetWorldRotation (Variables|Default|GetStaticMesh) (Math|Rotator|MakeRotator 0.0 0.0 1.8e+02) false false)
          (Transformation|AddWorldOffset (Variables|Default|GetStaticMesh) "0,120.000000,0.000000" false false))
        (:20
          (Components|StaticMesh|SetStaticMesh (Variables|Default|GetStaticMesh) "/Game/GreenwoodFantasyVillage/Meshes/SM_FenceBig_4m.SM_FenceBig_4m")
          (Transformation|SetWorldScale3D (Variables|Default|GetStaticMesh) (Math|Vector|MakeVector 1.25 1.25 1.25))
          (Transformation|SetWorldRotation (Variables|Default|GetStaticMesh) (Math|Rotator|MakeRotator 0.0 0.0 9e+01) false false)
          (Transformation|AddWorldOffset (Variables|Default|GetStaticMesh) "0.000000,-100.000000,0.000000" false false))
        (:21
          (Components|StaticMesh|SetStaticMesh (Variables|Default|GetStaticMesh) "/Game/GreenwoodFantasyVillage/Meshes/SM_Bench.SM_Bench")
          (Transformation|SetWorldScale3D (Variables|Default|GetStaticMesh) (Math|Vector|MakeVector 2.0 2.0 2.0))
          (Transformation|SetWorldRotation (Variables|Default|GetStaticMesh) (Math|Rotator|MakeRotator 0.0 0.0 (Math|Random|RandomFloatinRange 45.0 135.0)) false false :!label _label_9))
        (:22
          (Components|StaticMesh|SetStaticMesh (Variables|Default|GetStaticMesh) "/Game/GreenwoodFantasyVillage/Meshes/SM_Billboard.SM_Billboard")
          (Transformation|SetWorldScale3D (Variables|Default|GetStaticMesh) (Math|Vector|MakeVector 1.0 1.0 1.0))
          (goto _label_9))
        (:23
          (Components|StaticMesh|SetStaticMesh (Variables|Default|GetStaticMesh) "/Game/GreenwoodFantasyVillage/Meshes/SM_Boat.SM_Boat")
          (Transformation|SetWorldScale3D (Variables|Default|GetStaticMesh) (Math|Vector|MakeVector 1.0 1.0 1.0))
          (switch int (Math|Random|RandomIntegerinRange 0 1)
            (:0
              (Transformation|SetWorldRotation (Variables|Default|GetStaticMesh) (Math|Rotator|MakeRotator 0.0 0.0 (Math|Random|RandomFloatinRange 165.0 195.0)) false false))
            (:1
              (Transformation|SetWorldRotation (Variables|Default|GetStaticMesh) (Math|Rotator|MakeRotator 0.0 0.0 (Math|Random|RandomFloatinRange -15.0 15.0)) false false))))
        (:24
          (Components|StaticMesh|SetStaticMesh (Variables|Default|GetStaticMesh) "/Game/GreenwoodFantasyVillage/Meshes/SM_BushBig_A.SM_BushBig_A")
          (Transformation|SetWorldScale3D (Variables|Default|GetStaticMesh) (Math|Vector|MakeVector 1.0 1.0 1.0) :!label _label_10)
          (Transformation|SetWorldRotation (Variables|Default|GetStaticMesh) (Math|Rotator|MakeRotator 0.0 0.0 (Math|Random|RandomFloatinRange 0.0 3.6e+02)) false false))
        (:25
          (Components|StaticMesh|SetStaticMesh (Variables|Default|GetStaticMesh) "/Game/GreenwoodFantasyVillage/Meshes/SM_BushBig_B.SM_BushBig_B")
          (goto _label_10))
        (:26
          (Components|StaticMesh|SetStaticMesh (Variables|Default|GetStaticMesh) "/Game/GreenwoodFantasyVillage/Meshes/SM_BushBig_C.SM_BushBig_C")
          (goto _label_10))
        (:27
          (Components|StaticMesh|SetStaticMesh (Variables|Default|GetStaticMesh) "/Game/GreenwoodFantasyVillage/Meshes/SM_Barn.SM_Barn")
          (Transformation|SetWorldScale3D (Variables|Default|GetStaticMesh) (Math|Vector|MakeVector 0.5 0.5 0.5))
          (Transformation|SetWorldRotation (Variables|Default|GetStaticMesh) (Math|Rotator|MakeRotator 0.0 0.0 2.7e+02) false false))
        (:28
          (Components|StaticMesh|SetStaticMesh (Variables|Default|GetStaticMesh) "/Game/GreenwoodFantasyVillage/Meshes/SM_HouseB.SM_HouseB")
          (Transformation|SetWorldScale3D (Variables|Default|GetStaticMesh) (Math|Vector|MakeVector 0.75 0.75 0.75))
          (Transformation|SetWorldRotation (Variables|Default|GetStaticMesh) (Math|Rotator|MakeRotator 0.0 0.0 1.8e+02) false false))
        (:29
          (Components|StaticMesh|SetStaticMesh (Variables|Default|GetStaticMesh) "/Game/GreenwoodFantasyVillage/Meshes/SM_Mill.SM_Mill")
          (Transformation|SetWorldScale3D (Variables|Default|GetStaticMesh) (Math|Vector|MakeVector 0.75 0.75 0.75))
          (Transformation|SetWorldRotation (Variables|Default|GetStaticMesh) (Math|Rotator|MakeRotator 0.0 0.0 9e+01) false false))
        (:30
          (Components|StaticMesh|SetStaticMesh (Variables|Default|GetStaticMesh) "/Game/GreenwoodFantasyVillage/Meshes/SM_FenceSmallA_2m.SM_FenceSmallA_2m")
          (Transformation|SetWorldScale3D (Variables|Default|GetStaticMesh) (Math|Vector|MakeVector 1.0 1.0 1.0) :!label _label_11)
          (Transformation|SetWorldRotation (Variables|Default|GetStaticMesh) (Math|Rotator|MakeRotator 0.0 0.0 9e+01) false false))
        (:31
          (Components|StaticMesh|SetStaticMesh (Variables|Default|GetStaticMesh) "/Game/GreenwoodFantasyVillage/Meshes/SM_FenceSmallB_2m.SM_FenceSmallB_2m")
          (goto _label_11))))
    (:1
      (goto _label))
    (:2
      (Components|DestroyComponent (Variables|Default|GetStaticMesh))
      (switch int (Math|Random|RandomIntegerinRange 0 2)
        (:0
          (Class|SkinnedMeshComponent|SetSkeletalMesh (Variables|Default|GetSkeletalMesh) "/Game/UndeadPack/Zombie/Mesh/SK_Zombie.SK_Zombie" true)
          (CallFunction|ZombieSpawned))
        (:1
          (Class|SkinnedMeshComponent|SetSkeletalMesh (Variables|Default|GetSkeletalMesh) "/Game/UndeadPack/SkeletonEnemy/Mesh/SK_Skeleton.SK_Skeleton" true)
          (Transformation|SetWorldScale3D (Variables|Default|GetSkeletalMesh) (Math|Vector|MakeVector 2.0 2.0 2.0))
          (CallFunction|SkeletonSpawned))
        (:2
          (Class|SkinnedMeshComponent|SetSkeletalMesh (Variables|Default|GetSkeletalMesh) "/Game/UndeadPack/Ghoul/Mesh/SK_Ghoul_Full.SK_Ghoul_Full" true)
          (Transformation|SetWorldScale3D (Variables|Default|GetSkeletalMesh) (Math|Vector|MakeVector 2.0 2.0 2.0))
          (CallFunction|GhoulSpawned))))))

(fn ReturnParent
  (return (Variables|Default|GetParentRef)))

(fn SetParent
  (params (Parent :type BP%20Spawner%20Base%20Object%20Reference))
  (Variables|Default|SetParentRef Parent)
  (return false))