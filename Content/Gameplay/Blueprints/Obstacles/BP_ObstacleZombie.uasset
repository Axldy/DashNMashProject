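; BP_ObstacleZombie is a zombie obstacle that ends the game when a BP_PawnBase overlaps its skeletal mesh.
; The overlap calls HitObstacle on the pawn and GameOver on the level manager, if found, then plays one of two random attack animations before returning to looping idle after a fixed delay.
; SetParent and ReturnParent store and expose a parent reference.
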(event OnComponentBeginOverlap(SkeletalMesh)
  (params (OverlappedComponent :type Primitive%20Component%20Object%20Reference) (OtherActor :type Actor%20Object%20Reference) (OtherComp :type Primitive%20Component%20Object%20Reference) (OtherBodyIndex :type Integer) (bFromSweep :type Boolean) (SweepResult :type Hit%20Result%20Structure%20%28by%20ref%29))
  (bind (_levelmanager _levelmanagerfound) (CallFunction|GetLevelManager))
  (bind _asbp_pawn_base (Utilities|Casting|CastToBP_PawnBase OtherActor))
  (Default|HitObstacle _asbp_pawn_base)
  (if _levelmanagerfound
    (Default|GameOver _levelmanager)
    (switch int (Math|Random|RandomIntegerinRange 0 1)
      (:0
        (Components|Animation|PlayAnimation (Variables|Default|GetSkeletalMesh) "/Game/UndeadPack/Zombie/Animations/Anim_Attack1.Anim_Attack1" false)
        (Utilities|FlowControl|Delay 2.47))
      (:1
        (Components|Animation|PlayAnimation (Variables|Default|GetSkeletalMesh) "/Game/UndeadPack/Zombie/Animations/Anim_Attack2.Anim_Attack2" false)
        (Utilities|FlowControl|Delay 1.97)))
    (Components|Animation|PlayAnimation (Variables|Default|GetSkeletalMesh) "/Game/UndeadPack/Zombie/Animations/Anim_Idle.Anim_Idle" true)))

(fn ConstructionScript)

(fn ReturnParent
  (return (Variables|Default|GetParentRef)))

(fn SetParent
  (params (Parent :type BP%20Spawner%20Base%20Object%20Reference))
  (Variables|Default|SetParentRef Parent)
  (return false))